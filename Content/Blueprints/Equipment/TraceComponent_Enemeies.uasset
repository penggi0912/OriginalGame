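; Actor component that handles melee hit detection for enemy weapons.
; While the weapon is flagged active, each Tick runs a multi sphere trace between the "start" and "end" sockets on the referenced weapon's mesh, with debug drawing.
; Each newly hit actor takes the weapon's SwordDamage and joins an ignore list to prevent repeat hits; a comment says the pawn clears that list.
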(event `self.ReceiveTick`
  (params (DeltaSeconds :type "Float (single-precision)"))
  (bind _enemyweapon_ref (`self.EnemyWeapon_Ref`))
  ;[1 1 1] 武器のダメージ判定
  (if (`self.EenemyWeaponActive`)
    (`/Engine/EditorBlueprintResources/StandardMacros.IsValid` _enemyweapon_ref
      (:`Is Valid`
        (bind _outhits (`KismetSystemLibrary.SphereTraceMulti` :`Start` (`SceneComponent.GetSocketLocation` (`/Game/Blueprints/Equipment/BP_EnemySword.SkeletalMesh` _enemyweapon_ref) "start") :`End` (`SceneComponent.GetSocketLocation` (`/Game/Blueprints/Equipment/BP_EnemySword.SkeletalMesh` _enemyweapon_ref) "end") :`Radius` 12.0 :`TraceChannel` "TraceTypeQuery4" :`DrawDebugType` "ForDuration" :`DrawTime` 2.0))
        (for _array_element _outhits
          (bind (_bblockinghit _binitialoverlap _time _distance _location _impactpoint _normal _impactnormal _physmat _hitactor) (`GameplayStatics.BreakHitResult` _array_element))
          (if (not (`KismetArrayLibrary.Array_Contains` (`self.ActorToIgnore`) _hitactor))
            (`GameplayStatics.ApplyDamage` _hitactor (`/Game/Blueprints/Equipment/BP_EnemySword.SwordDamage` (`self.EnemyWeapon_Ref`))) ; SwordDamageに設定されたダメージを与える
            (`KismetArrayLibrary.Array_Add` (`self.ActorToIgnore`) _hitactor) ; ActorToIgnore変数の配列にダメージを格納、\nポーン側でクリア
          ))))))