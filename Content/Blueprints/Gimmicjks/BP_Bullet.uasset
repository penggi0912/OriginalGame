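; BP_Bullet is a physics-driven projectile that damages the first actor it hits.
; On BeginPlay it launches its static mesh along the actor's forward vector with a velocity-change impulse.
; Each tick an upward acceleration, blended by GravityScale, counteracts gravity to tune bullet drop.
; The first hit applies damage once, stops that tick compensation and makes the mesh ignore the Pawn channel.
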(event `self.ReceiveTick`
  (params (DeltaSeconds :type "Float (single-precision)"))
  ;[1 1 1] 弾丸の重力加速度調整
  (`PrimitiveComponent.AddForce` (`self.StaticMeshComponent`) (`KismetMathLibrary.VLerp` (0.0 0.0 980.0) (0.0 0.0 0.0) (`self.GravityScale`)) "None" true))

(event `self.ReceiveHit`
  (params (MyComp :type "PrimitiveComponent Object Reference") (Other :type "Actor Object Reference") (OtherComp :type "PrimitiveComponent Object Reference") (bSelfMoved :type Boolean) (HitLocation :type "Vector Structure") (HitNormal :type "Vector Structure") (NormalImpulse :type "Vector Structure") (Hit :type "HitResult Structure (by ref)"))
  ;[1 1 1] ダメージ処理(1 Kill)
  (`/Engine/EditorBlueprintResources/StandardMacros.DoOnce` false
    (:`Completed`
      (`GameplayStatics.ApplyDamage` Other 1.0 null self)
      (`self.SetActorTickEnabled` false)
      (`PrimitiveComponent.SetCollisionResponseToChannel` (`self.StaticMeshComponent`) "ECC_Pawn" "ECR_Ignore"))))

(event `self.ReceiveBeginPlay`
  ;[1 1 1] 弾丸発射速度
  (`PrimitiveComponent.AddImpulse` (`self.StaticMeshComponent`) (* (`self.GetActorForwardVector`) (`self.BulletInitialSpeed`)) "None" true) ; 弾丸を初速度で弾き出す
)

(fn `UserConstructionScript`)