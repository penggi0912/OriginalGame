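; Turret gimmick that fires a burst of bullets with a spinning barrel when its Sensor check succeeds.
; Tick polls the Sensor and starts a DoOnce-guarded timeline that drives only the Barrel's roll through RotatingMovement, re-arming when finished.
; The timeline's Fire events alternately start and clear, via FlipFlop, a looping timer paced by FireRate.
; Each timer tick spawns BP_Bullet at the Muzzle socket with random yaw spread and prints debug text.
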(event `self.ReceiveBeginPlay`
  ;[1 1 1] 銃身のみ回転
  (`MovementComponent.SetUpdatedComponent` (`self.RotatingMovement`) (`self.Barrel`)))

(event `StartFire`
  (bind _returnvalue (`KismetMathLibrary.SafeDivide` 1.2 (`self.FireRate`)))
  ;[1 1 1] 弾丸発射
  (`/Engine/EditorBlueprintResources/StandardMacros.DoOnce` false :!label _label
    (:`Completed`
      (bind (_direction _muzzlerolling) (`Timeline|FireControlTL` :!via `PlayFromStart`)
        (:`Update`
          (set `RotatingMovementComponent.RotationRate` (`KismetMathLibrary.MakeRotator` _muzzlerolling) (`self.RotatingMovement`)))
        (:`Finished`
          (goto _label :!via `Reset`))
        (:`Fire`
          (`/Engine/EditorBlueprintResources/StandardMacros.FlipFlop` ; A：射撃開始\nB：射撃終了
            (:`A`
              (bind _returnvalue_2 (`KismetSystemLibrary.K2_SetTimerDelegate` (delegate `Fire`) _returnvalue true (* _returnvalue -1.0))))
            (:`B`
              (`KismetSystemLibrary.K2_ClearAndInvalidateTimerHandle` _returnvalue_2))))))))

(event `Fire`
  ;[1 1 1] 弾丸発射
  (`KismetSystemLibrary.DrawDebugString` (0.0 0.0 0.0) "Fire!" self (struct :`R` 1.0 :`G` 1.0 :`B` 1.0 :`A` 1.0) 0.2) ; Fireのデバッグ
  (`|SpawnActorFromClass` "/Game/Blueprints/Gimmicjks/BP_Bullet.BP_Bullet_C" (`KismetMathLibrary.ComposeTransforms` (`self.GetLocalSpread`) (`self.GetMuzzleTransform`)) "Undefined" "MultiplyWithRoot" null 600.0 0.2 null) ; BP_Bulletをスポーン
)

(event `self.ReceiveTick`
  (params (DeltaSeconds :type "Float (single-precision)"))
  ;[1 1 1] センサー呼び出し&アクタにHitしたら弾丸発射
  (bind (_outactors _return_value) (`/Game/Blueprints/Components/AC_Sensor.CheckSensor` (`self.Sensor`)))
  (if _return_value
    (`self.StartFire`)))

(fn `GetLocalSpread`
  (returns (ReturnValue :type "Transform Structure"))
  ;[1 1 1] 銃口のぶれのトランスフォームを作成
  (return (`KismetMathLibrary.MakeTransform` (0.0 0.0 0.0) (`KismetMathLibrary.MakeRotator` 0.0 0.0 (`KismetMathLibrary.RandomFloatInRange` -10.0 10.0)))))

(fn `GetMuzzleTransform`
  (returns (ReturnValue :type "Transform Structure"))
  (return (`SceneComponent.GetSocketTransform` (`self.StaticMeshComponent`) "Muzzle" "RTS_World")))

(fn `UserConstructionScript`)