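; Skeleton enemy pawn with a sword, HP bar, montage-driven combat, lock-on targetability and walk/sprint speed toggles.
; BeginPlay attaches the sword, links it to the trace component, then replays one attack montage every second; the behavior tree call is unwired.
; Damage updates the bar and plays a hit reaction, or at zero HP stops AI, movement and collision before timed removal.
; Attack plays a random montage, storing its length; ClearEnemies resets trace ignores between swings.
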(event `self.ReceiveBeginPlay`
  ;[1 1 1] AI System
  ;[1 1 1] 武器装着
  (bind _returnvalue (`|SpawnActorFromClass` "/Game/Blueprints/Equipment/BP_EnemySword.BP_EnemySword_C" (`SceneComponent.GetSocketTransform` (`self.Mesh`) "weapon_r" "RTS_World") "Undefined" "MultiplyWithRoot" null null))
  (bind _output_get (set `self.EnemyWeaponref` _returnvalue))
  (`self.K2_AttachToComponent` _output_get (`self.Mesh`) "weapon_r" "SnapToTarget" "SnapToTarget" "SnapToTarget" true)
  (set `/Game/Blueprints/Equipment/TraceComponent_Enemeies.EnemyWeapon_Ref` (`self.EnemyWeaponref`) (`self.TraceComponent_Enemeies`))
  ;[1 1 1] HPバーウィジェット呼び出し
  (bind _aswbp_enemy_hp_bar (cast `/Game/Blueprints/Widget/WBP_EnemyHP_Bar` (`WidgetComponent.GetWidget` (`self.HP_Bar`))))
  (bind _output_get_2 (set `self.As WBP Enemy HP Bar` _aswbp_enemy_hp_bar))
  (set `/Game/Blueprints/Widget/WBP_EnemyHP_Bar.Enemy_ref` self _output_get_2)
  (bind _returnvalue_2 (`self.PlayAnimMontage` "/Game/Animation/Enemies/Skele_AttackC_Montage.Skele_AttackC_Montage" :!label _label))
  (set `self.AttackLength` _returnvalue_2) ; 攻撃間隔として、攻撃アニメモンタージュの\n長さをAttackLength変数にセット
  (`KismetSystemLibrary.Delay` 1.0)
  (goto _label))

(event `self.ReceiveAnyDamage`
  (params (Damage :type "Float (single-precision)") (DamageType :type "DamageType Object Reference") (InstigatedBy :type "Controller Object Reference") (DamageCauser :type "Actor Object Reference"))
  (bind _hp_bar (`self.HP_Bar`))
  ;[1 1 1] 非ダメージ/死亡時の処理
  (bind _output_get (set `self.HP` (- (`self.HP`) Damage)))
  (`KismetSystemLibrary.PrintString` (`KismetStringLibrary.Concat_StrStr` "残りHP：" (`KismetStringLibrary.Conv_DoubleToString` _output_get)) true true (struct :`R` 1.0 :`G` 0.126427 :`B` 0.246205 :`A` 1.0)) ; デバッグ用残りHP表示
  (if (<= _output_get 0.0)
    (`SceneComponent.SetVisibility` _hp_bar false false) ; HPバー非表示
    (`/Engine/EditorBlueprintResources/StandardMacros.DoOnce` false ; 死亡処理は一度だけ実行
      (:`Completed`
        (`BrainComponent.StopLogic` (`AIController.BrainComponent` (`AIBlueprintHelperLibrary.GetAIController` self)) "") ; 死亡後に動かないようロジック停止
        (`self.PlayAnimMontage` "/Game/Animation/Enemies/Skele_Death_Montage.Skele_Death_Montage")
        (`CharacterMovementComponent.DisableMovement` (`self.CharacterMovement`)) ; キャラクターを動けなくする
        (`self.SetLifeSpan` self 5.0)
        (`self.SetLifeSpan` (`self.EnemyWeaponref`) 5.0) ; 5秒の寿命をつける
        (`PrimitiveComponent.SetCollisionProfileName` (`self.CapsuleComponent`) "NoCollision" true) ; 死亡後に残ったカプセルコンポーネントが余計な\nHit判定を起こさないようにコリジョンプロファイルを変更
        (`KismetSystemLibrary.PrintString` (`KismetStringLibrary.Concat_StrStr` "コリジョン名：" (`KismetStringLibrary.Conv_NameToString` (`PrimitiveComponent.GetCollisionProfileName` (`self.CapsuleComponent`))))) ; デバッグ用コリジョン名表示
      ))
    (else
      (`SceneComponent.SetVisibility` _hp_bar true false) ; HPバー表示
      (`/Game/Blueprints/Widget/WBP_EnemyHP_Bar.Update HP Bar` (`self.As WBP Enemy HP Bar`)) ; HPバー更新
      (`self.PlayAnimMontage` "/Game/Animation/Enemies/Skele_Hit_Montage.Skele_Hit_Montage"))))

(event `Attack`
  ;[1 1 1] 攻撃
  (bind _returnvalue (`self.PlayAnimMontage` (`KismetArrayLibrary.Array_Random` (`self.AttackAnimation`))))
  (set `self.AttackLength` _returnvalue) ; 攻撃間隔として、攻撃アニメモンタージュの\n長さをAttackLength変数にセット
)

(event `Clear Enemies`
  ;[1 1 1] トレースの当たり判定配列をクリア
  ; (二撃目以降の攻撃を有効化)
  (`KismetArrayLibrary.Array_Clear` (`/Game/Blueprints/Equipment/TraceComponent_Enemeies.ActorToIgnore` (`self.TraceComponent_Enemeies`))))

(fn `BeginSprint`
  (returns (Succeed :type Boolean))
  (bind _charactermovement (`self.CharacterMovement`))
  (if (`self.IsSprinting`)
    (return false) ; 失敗を返す
    (else
      (set `CharacterMovementComponent.MaxWalkSpeed` (`CharacterMovementComponent.MaxWalkSpeed` _charactermovement) _charactermovement) ; スプリント速度を設定
      (set `self.IsSprinting` true) ; スプリント状態になったら
      (return true) ; 成功を返す
    )))

(fn `BeginWalk`
  (returns (Succeed :type Boolean))
  (bind _charactermovement (`self.CharacterMovement`))
  (if (`self.Is Walking`)
    (return false) ; 失敗を返す
    (else
      (set `CharacterMovementComponent.MaxWalkSpeed` (`CharacterMovementComponent.MaxWalkSpeedCrouched` _charactermovement) _charactermovement) ; 歩行速度を設定
      (set `self.Is Walking` true) ; 歩行状態になった
      (return true) ; 成功を返す
    )))

(fn `EndSprint`
  (returns (Succeed :type Boolean))
  (bind _charactermovement (`self.CharacterMovement`))
  (if (`self.IsSprinting`)
    (set `CharacterMovementComponent.MaxWalkSpeed` (/ (`CharacterMovementComponent.MaxWalkSpeed` _charactermovement) 2.0) _charactermovement) ; 通常歩行時の速度を設定
    (set `self.IsSprinting` false) ; スプリント状態でない
    (return true)
    (else
      (return false) ; 失敗を返す
    )))

(fn `EndWalk`
  (returns (Succeed :type Boolean))
  (if (`self.Is Walking`)
    (set `CharacterMovementComponent.MaxWalkSpeed` 1000.0 (`self.CharacterMovement`)) ; 通常移動時の速度を設定
    (set `self.Is Walking` false) ; 歩行状態でない
    (return true)
    (else
      (return false) ; 失敗を返す
    )))

(fn `Get Is Sprinting`
  (returns (ReturnValue :type Boolean))
  (return (`self.Is Walking`)))

(fn `IsTargetable`
  (returns (ReturnValue :type Boolean))
  (if (< (`self.HP`) 1.0)
    (return false)
    (else
      (return true))))

(fn `UserConstructionScript`)