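; BP_Pawn is a character that tells floor actors when it steps onto or off them.
; Each Tick compares the floor actor from CharacterMovement's current floor hit result with the cached LastFloor.
; On a change, it sends OnPawnOff to the old floor and OnPawnOn to the new one through the BI_Floor interface, then updates LastFloor.
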(event `self.ReceiveTick`
  (params (DeltaSeconds :type "Float (single-precision)"))
  (bind _floor (`self.GetCurrentFloor`))
  ;[1 1 1] 床認識機能
  (if (!= (`self.GetCurrentFloor`) (`self.Last Floor`))
    (`|ExecutionSequence`
      (:`then_0`
        (bind _asbi_floor (cast `/Game/Blueprints/Interfaces/BI_Floor` (`self.Last Floor`)))
        (`/Game/Blueprints/Interfaces/BI_Floor.OnPawnOff` _asbi_floor self) ; さっきまで踏んでいた床から\n降りたことを通知
      )
      (:`then_1`
        (bind _asbi_floor_2 (cast `/Game/Blueprints/Interfaces/BI_Floor` _floor))
        (`/Game/Blueprints/Interfaces/BI_Floor.OnPawnOn` _asbi_floor_2 self) ; 現在の床を踏み始めたことを通知
      )
      (:`then_2`
        (set `self.Last Floor` _floor) ; 「さっきまで踏んでいた床」の変数を\n「現在の床」に更新
      ))))

(fn `GetCurrentFloor`
  (returns (Floor :type "Actor Object Reference"))
  (return (`.HitActor` (`GameplayStatics.BreakHitResult` (`.HitResult` (break `FindFloorResult` (`CharacterMovementComponent.CurrentFloor` (`self.CharacterMovement`))))))))

(fn `UserConstructionScript`)