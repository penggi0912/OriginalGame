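; Spline-placed row of street power posts with lights and connecting cables, built entirely in the construction script.
; Spawns BP_Power_Post child actors along the spline points, matching their rotation.
; Snaps each post's five cables to the next post's connectors, sizing lengths by connector distance, and zeroes cables and hides the lamp on the final entry.
; Per-index arrays set lamp yaw, spotlight intensity and radius, light color and matching emissive material color.
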(fn `UserConstructionScript`
  (bind _post_spawn_loop_index (`self.Post Spawn Loop Index`))
  (bind _spline (`self.Spline`))
  (bind _output (`|GetArrayItem` (`self.PowerPost Child Actor Refrences`) (`self.Cable Attach Loop Index`)))
  (bind _output_2 (`|GetArrayItem` (`self.PowerPost Child Actor Refrences`) (+ (`self.Cable Attach Loop Index`) 1)))
  (bind _cable_1 (`/Game/Imports/Downtown_Alley/Blueprints/BP_Power_Post.Cable 1` _output))
  (bind _cable_2 (`/Game/Imports/Downtown_Alley/Blueprints/BP_Power_Post.Cable 2` _output))
  (bind _cable_3 (`/Game/Imports/Downtown_Alley/Blueprints/BP_Power_Post.Cable 3` _output))
  (bind _cable_4 (`/Game/Imports/Downtown_Alley/Blueprints/BP_Power_Post.Cable 4` _output))
  (bind _cable_5 (`/Game/Imports/Downtown_Alley/Blueprints/BP_Power_Post.Cable 5` _output))
  (bind _con_1 (`/Game/Imports/Downtown_Alley/Blueprints/BP_Power_Post.Con 1` _output_2))
  (bind _con_2 (`/Game/Imports/Downtown_Alley/Blueprints/BP_Power_Post.Con 2` _output_2))
  (bind _con_3 (`/Game/Imports/Downtown_Alley/Blueprints/BP_Power_Post.Con 3` _output_2))
  (bind _con_4 (`/Game/Imports/Downtown_Alley/Blueprints/BP_Power_Post.Con 4` _output_2))
  (bind _con_5 (`/Game/Imports/Downtown_Alley/Blueprints/BP_Power_Post.Con 5` _output_2))
  (set `self.Number Of Spline Points` (`SplineComponent.GetNumberOfSplinePoints` (`self.Spline`)))
  (for _index (range (+ (`self.Number Of Spline Points`) 1))
    (set `self.Post Spawn Loop Index` _index)
    (bind _returnvalue (`AddComponent|NODE_AddChildActorComponent-1` :`RelativeTransform` (`KismetMathLibrary.Conv_VectorToTransform` (`SplineComponent.GetLocationAtSplinePoint` _spline _post_spawn_loop_index "Local"))))
    (`ChildActorComponent.SetChildActorClass` _returnvalue "/Game/Imports/Downtown_Alley/Blueprints/BP_Power_Post.BP_Power_Post_C")
    (bind _childactor (`ChildActorComponent.ChildActor` _returnvalue))
    (bind _asbp_power_post (cast `/Game/Imports/Downtown_Alley/Blueprints/BP_Power_Post` _childactor))
    (`KismetArrayLibrary.Array_Add` (`self.PowerPost Child Actor Refrences`) _asbp_power_post)
    (`SceneComponent.K2_SetRelativeRotation` (`Actor.RootComponent` _childactor) (`SplineComponent.GetRotationAtSplinePoint` _spline _post_spawn_loop_index "Local") false false))
  (for _index_2 (range (+ (`self.Number Of Spline Points`) 1))
    (set `self.Cable Attach Loop Index` _index_2)
    (`|ExecutionSequence`
      (:`then_0`
        (`SceneComponent.K2_AttachToComponent` _cable_1 _con_1 "None" "SnapToTarget" "SnapToTarget" "KeepWorld" true)
        (set `CableComponent.CableLength` (`KismetMathLibrary.VSize` (- (`SceneComponent.K2_GetComponentLocation` (`/Game/Imports/Downtown_Alley/Blueprints/BP_Power_Post.Con 1` _output)) (`SceneComponent.K2_GetComponentLocation` _con_1))) _cable_1)
        (set `CableComponent.CableLength` 0.0 (`/Game/Imports/Downtown_Alley/Blueprints/BP_Power_Post.Cable 1` (`|GetArrayItem` (`self.PowerPost Child Actor Refrences`) (`self.Number Of Spline Points`)))))
      (:`then_1`
        (`SceneComponent.K2_AttachToComponent` _cable_2 _con_2 "None" "SnapToTarget" "SnapToTarget" "KeepWorld" true)
        (set `CableComponent.CableLength` (* (`KismetMathLibrary.VSize` (- (`SceneComponent.K2_GetComponentLocation` (`/Game/Imports/Downtown_Alley/Blueprints/BP_Power_Post.Con 2` _output)) (`SceneComponent.K2_GetComponentLocation` _con_2))) 1.025) _cable_2)
        (set `CableComponent.CableLength` 0.0 (`/Game/Imports/Downtown_Alley/Blueprints/BP_Power_Post.Cable 2` (`|GetArrayItem` (`self.PowerPost Child Actor Refrences`) (`self.Number Of Spline Points`)))))
      (:`then_2`
        (`SceneComponent.K2_AttachToComponent` _cable_3 _con_3 "None" "SnapToTarget" "SnapToTarget" "KeepWorld" true)
        (set `CableComponent.CableLength` (* (`KismetMathLibrary.VSize` (- (`SceneComponent.K2_GetComponentLocation` (`/Game/Imports/Downtown_Alley/Blueprints/BP_Power_Post.Con 3` _output)) (`SceneComponent.K2_GetComponentLocation` _con_3))) 0.96) _cable_3)
        (set `CableComponent.CableLength` 0.0 (`/Game/Imports/Downtown_Alley/Blueprints/BP_Power_Post.Cable 3` (`|GetArrayItem` (`self.PowerPost Child Actor Refrences`) (`self.Number Of Spline Points`)))))
      (:`then_3`
        (`SceneComponent.K2_AttachToComponent` _cable_4 _con_4 "None" "SnapToTarget" "SnapToTarget" "KeepWorld" true)
        (set `CableComponent.CableLength` (`KismetMathLibrary.VSize` (- (`SceneComponent.K2_GetComponentLocation` (`/Game/Imports/Downtown_Alley/Blueprints/BP_Power_Post.Con 4` _output)) (`SceneComponent.K2_GetComponentLocation` _con_4))) _cable_4)
        (set `CableComponent.CableLength` 0.0 (`/Game/Imports/Downtown_Alley/Blueprints/BP_Power_Post.Cable 4` (`|GetArrayItem` (`self.PowerPost Child Actor Refrences`) (`self.Number Of Spline Points`)))))
      (:`then_4`
        (`SceneComponent.K2_AttachToComponent` _cable_5 _con_5 "None" "SnapToTarget" "SnapToTarget" "KeepWorld" true)
        (set `CableComponent.CableLength` (`KismetMathLibrary.VSize` (- (`SceneComponent.K2_GetComponentLocation` (`/Game/Imports/Downtown_Alley/Blueprints/BP_Power_Post.Con 5` _output)) (`SceneComponent.K2_GetComponentLocation` _con_5))) _cable_5)
        (set `CableComponent.CableLength` 0.0 (`/Game/Imports/Downtown_Alley/Blueprints/BP_Power_Post.Cable 5` (`|GetArrayItem` (`self.PowerPost Child Actor Refrences`) (`self.Number Of Spline Points`)))))))
  (for _index_3 (range (+ (`self.Number Of Spline Points`) 1))
    (`SceneComponent.K2_AddLocalRotation` (`/Game/Imports/Downtown_Alley/Blueprints/BP_Power_Post.Power_Post_Light` (`|GetArrayItem` (`self.PowerPost Child Actor Refrences`) _index_3)) (`KismetMathLibrary.MakeRotator` 0.0 0.0 (`|GetArrayItem` (`self.Light Pole Rotation`) _index_3)) false false)
    (`SceneComponent.SetVisibility` (`/Game/Imports/Downtown_Alley/Blueprints/BP_Power_Post.Power_Post_Light` (`|GetArrayItem` (`self.PowerPost Child Actor Refrences`) (`self.Number Of Spline Points`))) false false)
    (`SceneComponent.SetVisibility` (`/Game/Imports/Downtown_Alley/Blueprints/BP_Power_Post.SpotLight` (`|GetArrayItem` (`self.PowerPost Child Actor Refrences`) (`self.Number Of Spline Points`))) false false))
  (for _index_4 (range (+ (`self.Number Of Spline Points`) 1))
    (`LightComponent.SetIntensity` (`/Game/Imports/Downtown_Alley/Blueprints/BP_Power_Post.SpotLight` (`|GetArrayItem` (`self.PowerPost Child Actor Refrences`) _index_4)) (`|GetArrayItem` (`self.Light Intensity`) _index_4)))
  (for _index_5 (range (+ (`self.Number Of Spline Points`) 1))
    (`LightComponent.SetLightColor` (`/Game/Imports/Downtown_Alley/Blueprints/BP_Power_Post.SpotLight` (`|GetArrayItem` (`self.PowerPost Child Actor Refrences`) _index_5)) (`|GetArrayItem` (`self.Light Color`) _index_5) true)
    (`LightComponent.SetLightColor` (`/Game/Imports/Downtown_Alley/Blueprints/BP_Power_Post.PointLight` (`|GetArrayItem` (`self.PowerPost Child Actor Refrences`) _index_5)) (`|GetArrayItem` (`self.Light Color`) _index_5) true))
  (for _index_6 (range (+ (`self.Number Of Spline Points`) 1))
    (`PointLightComponent.SetAttenuationRadius` (`/Game/Imports/Downtown_Alley/Blueprints/BP_Power_Post.SpotLight` (`|GetArrayItem` (`self.PowerPost Child Actor Refrences`) _index_6)) (`|GetArrayItem` (`self.Light Radius`) _index_6)))
  (for _index_7 (range (+ (`self.Number Of Spline Points`) 1))
    (`MeshComponent.SetVectorParameterValueOnMaterials` (`/Game/Imports/Downtown_Alley/Blueprints/BP_Power_Post.Power_Post_Light` (`|GetArrayItem` (`self.PowerPost Child Actor Refrences`) _index_7)) "Emissive Color" (`KismetMathLibrary.Conv_LinearColorToVector` (`|GetArrayItem` (`self.Light Color`) _index_7)))))