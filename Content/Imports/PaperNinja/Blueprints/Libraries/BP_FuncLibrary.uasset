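; BP_FuncLibrary is a function library of small gameplay and math helpers in PaperNinja.
; CalcRay turns an origin, direction and length into ray start and end points.
; IsPlayerPawn reports whether an actor is a pawn possessed by a PlayerController.
; SineCurve evaluates a sine wave from amplitude, period, time and phase through a math expression, using a safe divide to derive angular frequency from the period.
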(fn CalcRay
  (params (Origin :type Vector) (Direction :type Vector) (Length :type Float%20%28double-precision%29))
  ;[1 1 1] 光線の計算
  (return Origin (+ Origin (* Direction Length))))

(fn IsPlayerPawn
  (params (Actor :type Actor%20Object%20Reference))
  ;[1 1 1] 自機判定
  (bind _aspawn (Utilities|Casting|CastToPawn Actor) ; アクタがポーンかどうかを判定
    (:then
      (Utilities|Casting|CastToPlayerController (Pawn|GetController _aspawn) ; 自機かどうかを判定
        (:then
          (return true))
        (:CastFailed
          _)))
    (:CastFailed
      _))
  (return false))

(fn SineCurve
  (params (Amplitude :type Float%20%28double-precision%29) (Period :type Float%20%28double-precision%29) (Time :type Float%20%28double-precision%29) (Phase :type Float%20%28double-precision%29))
  ;[1 1 1] A sin(2π/T*t+θ)で正弦波を計算
  (return (|(A*(sin(((w*t)+theta)))) Amplitude (Math|Float|SafeDivide (Math|Float|MultiplybyPi 2.0) Period) Time Phase)))