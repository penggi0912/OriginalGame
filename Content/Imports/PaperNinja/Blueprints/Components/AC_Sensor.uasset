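; AC_Sensor is a vision sensor component that finds actors inside a view cone from its attachment point.
; CheckSensor sweeps a box sized from sight length and angle along the forward vector, then filters hits through CanSeeActor.
; CanSeeActor requires the actor's location to pass IsInSight's dot-product angle test and a line trace to hit that actor first.
; CheckSensor returns the visible actors and whether any exist, drawing debug traces and cone.
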(fn `CanSeeActor`
  (params (TargetActor :type "Actor Object Reference"))
  (returns (ReturnValue :type Boolean))
  (bind _returnvalue (`Actor.K2_GetActorLocation` TargetActor))
  ;[1 1 1] ターゲットのアクタにライントレースが通るかを判定
  (if (`self.IsInSight` _returnvalue)
    (bind _outhit (`KismetSystemLibrary.LineTraceSingle` :`Start` (`self.K2_GetComponentLocation`) :`End` _returnvalue :`TraceChannel` "TraceTypeQuery3" :`DrawDebugType` "ForOneFrame")) ; ライントレース照射
    (return (== TargetActor (`.HitActor` (`GameplayStatics.BreakHitResult` _outhit))))
    (else
      (return false))))

(fn `CheckSensor`
  (returns (OutActors :type "Array of Actor Object Reference") (`Return Value` :type Boolean))
  (locals (ReturnActors :type "Array of Actor Object Reference"))
  (bind _returnactors (`local.ReturnActors`))
  (bind _location (.location (`self.K2_GetComponentToWorld`)))
  (bind _rotation (.rotation (`self.K2_GetComponentToWorld`)))
  (bind _returnvalue (* (`self.SightAngle`) 0.5))
  (bind _returnvalue_2 (`KismetMathLibrary.GetForwardVector` _rotation))
  (bind (_start _end) (`/Game/Imports/PaperNinja/Blueprints/Libraries/BP_FuncLibrary.CalcRay` _location _returnvalue_2 (`self.SightLength`)))
  (bind _returnvalue_3 (* (`self.SightLength`) (`KismetMathLibrary.DegTan` (* (`self.SightAngle`) 0.5))))
  ;[1 1 1] コンポーネントの取り付け位置からトレースを飛ばす
  (bind _outhits (`KismetSystemLibrary.BoxTraceMulti` :`Start` _start :`End` _end :`HalfSize` (`KismetMathLibrary.MakeVector` 1.0 _returnvalue_3 _returnvalue_3) :`Orientation` _rotation :`TraceChannel` "TraceTypeQuery4" :`DrawDebugType` "ForOneFrame")) ; ボックストレース照射
  (`KismetSystemLibrary.DrawDebugConeInDegrees` _location _returnvalue_2 (`self.SightLength`) _returnvalue _returnvalue 6 (struct :`R` 1.0 :`G` 0.167448 :`B` 0.976391 :`A` 1.0) 0.1 1.0)
  ;[1 1 1] 視界に入ったアクタをすべて配列に入れて返す
  (for _array_element _outhits
    (bind (_bblockinghit _binitialoverlap _time _distance _location_2 _impactpoint _normal _impactnormal _physmat _hitactor) (`GameplayStatics.BreakHitResult` _array_element))
    (bind _returnvalue_4 (`self.CanSeeActor` _hitactor)) ; ターゲットのアクタにライントレースが通るかを判定\nトレースチャンネル：Sight
    (if _returnvalue_4
      (`KismetArrayLibrary.Array_Add` (`local.ReturnActors`) _hitactor)))
  (return _returnactors (`KismetArrayLibrary.Array_IsNotEmpty` _returnactors)))

(fn `IsInSight`
  (params (TargetLocation :type "Vector Structure"))
  (returns (ReturnValue :type Boolean))
  ;[1 1 1] TargetLocationがSightAngleの内側にあるならTrue
  (return (<= (`KismetMathLibrary.DegAcos` (`KismetMathLibrary.Dot_VectorVector` (`KismetMathLibrary.GetDirectionUnitVector` (`self.K2_GetComponentLocation`) TargetLocation) (`self.GetForwardVector`))) (* (`self.SightAngle`) 0.5))))