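; Playable character pawn with camera-relative movement, look, sprint on the guard input, and a jump that winds up briefly via an animation transition event when standing still.
; Any damage, including force-kill, triggers one-time death: ragdoll with backflip impulse and timed despawn.
; Hits damage the other actor, and Tick compares the current floor to the last, notifying both through BI_Floor.
; The construction script attaches an optional weapon mesh to a socket.
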(event `self.OnJumped`
  (`self.OnPawnJumped`))

(event `self.ReceiveAnyDamage`
  (params (Damage :type "Float (single-precision)") (DamageType :type "DamageType Object Reference") (InstigatedBy :type "Controller Object Reference") (DamageCauser :type "Actor Object Reference"))
  (bind _mesh (`self.Mesh`))
  ;[1 1 1] ダメージ処理_死亡
  (`/Engine/EditorBlueprintResources/StandardMacros.DoOnce` false ; 死亡処理は一度だけ実行
    (:`Completed`
      (`KismetSystemLibrary.PrintString` "Died!")
      (`CharacterMovementComponent.DisableMovement` (`self.CharacterMovement`)) ; キャラクターを動けなくする
      (`self.SetLifeSpan` 5.0) ; 5秒の寿命をつける
      ;[1 1 1] ラグドール処理
      (`PrimitiveComponent.SetCollisionProfileName` _mesh "Ragdoll" true) ; ラグドール処理時にメッシュコンポーネントの\nプロファイルをラグドールに変更
      (`SkeletalMeshComponent.SetAllBodiesSimulatePhysics` _mesh true)
      ;[1 1 1] 死亡時、インパクトにより吹き飛ぶ処理
      (`SkeletalMeshComponent.AddImpulseToAllBodiesBelow` _mesh (-200.0 0.0 500.0) "None" true true) ; 後ろと上方向にインパクト
      (`PrimitiveComponent.AddAngularImpulseInDegrees` _mesh (0.0 -3600.0 0.0) "None" true) ; 足に撃力を与えて後転させる
      (`PrimitiveComponent.SetCollisionProfileName` (`self.CapsuleComponent`) "Spectator" true) ; ラグドール処理後に残ったカプセルコンポーネントが余計な\nHit判定を起こさないようにコリジョンプロファイルを変更
    )))

(event `self.ReceiveHit`
  (params (MyComp :type "PrimitiveComponent Object Reference") (Other :type "Actor Object Reference") (OtherComp :type "PrimitiveComponent Object Reference") (bSelfMoved :type Boolean) (HitLocation :type "Vector Structure") (HitNormal :type "Vector Structure") (NormalImpulse :type "Vector Structure") (Hit :type "HitResult Structure (by ref)"))
  ;[1 1 1] Hit相手にダメージを適用
  (`GameplayStatics.ApplyDamage` Other 1.0 null self))

(event `self.ReceiveTick`
  (params (DeltaSeconds :type "Float (single-precision)"))
  (bind _floor (`self.GetCurrentFloor`))
  ;[1 1 1] 床認識機能
  (if (!= (`self.GetCurrentFloor`) (`self.LastFloor`))
    (`|ExecutionSequence`
      (:`then_0`
        (bind _asbi_floor (cast `/Game/InGame/Blueprints/Interfaces/BI_Floor` (`self.LastFloor`)))
        (`/Game/InGame/Blueprints/Interfaces/BI_Floor.OnPawnOff` _asbi_floor self) ; さっきまで踏んでいた床から\n降りたことを通知
      )
      (:`then_1`
        (bind _asbi_floor_2 (cast `/Game/InGame/Blueprints/Interfaces/BI_Floor` _floor))
        (`/Game/InGame/Blueprints/Interfaces/BI_Floor.OnPawnOn` _asbi_floor_2 self) ; 現在の床を踏み始めたことを通知
      )
      (:`then_2`
        (set `self.LastFloor` _floor) ; 「さっきまで踏んでいた床」の変数を\n「現在の床」に更新
      ))))

(event `EnhancedInput|/Game/InGame/AI/Input/Actions/IA_Jump`
  (params (ActionValue :type Boolean) (ElapsedSeconds :type "Float (double-precision)") (TriggeredSeconds :type "Float (double-precision)") (InputAction :type "InputAction Object Reference" :default "/Game/InGame/AI/Input/Actions/IA_Jump.IA_Jump"))
  ;[1 1 1] ジャンプ操作の制御。静止時はタメジャンプ
  (:`Triggered`
    (if (`self.CanJump`)
      (if (not (>= (`KismetMathLibrary.VSizeXY` (`self.GetVelocity`)) 10.0))
        (`AnimInstance.RequestTransitionEvent` (`SkeletalMeshComponent.GetAnimInstance` (`self.Mesh`)) "StartJump" 0.1 "Shared" "Append")
        (`KismetSystemLibrary.Delay` 0.3) ; 0.3秒タメる
      )
      (`self.Jump`))))

(event `EnhancedInput|/Game/InGame/AI/Input/Actions/IA_Guard`
  (params (ActionValue :type Boolean) (ElapsedSeconds :type "Float (double-precision)") (TriggeredSeconds :type "Float (double-precision)") (InputAction :type "InputAction Object Reference" :default "/Game/InGame/AI/Input/Actions/IA_Guard.IA_Guard"))
  ;[1 1 1] 移動スピード
  (:`Triggered`
    (`self.BeginSprint`))
  (:`Completed`
    (`self.EndSprint`)))

(event `EnhancedInput|/Game/InGame/AI/Input/Actions/IA_ForceKill`
  (params (ActionValue :type Boolean) (ElapsedSeconds :type "Float (double-precision)") (TriggeredSeconds :type "Float (double-precision)") (InputAction :type "InputAction Object Reference" :default "/Game/InGame/AI/Input/Actions/IA_ForceKill.IA_ForceKill"))
  ;[1 1 1] 強制Kill
  (:`Triggered`
    (`GameplayStatics.ApplyDamage` self 1.0 null self)))

(event `EnhancedInput|/Game/InGame/AI/Input/Actions/IA_Look`
  (params (ActionValue :type "Vector2D Structure") (ElapsedSeconds :type "Float (double-precision)") (TriggeredSeconds :type "Float (double-precision)") (InputAction :type "InputAction Object Reference" :default "/Game/InGame/AI/Input/Actions/IA_Look.IA_Look"))
  (bind (_x _y) (`KismetMathLibrary.BreakVector2D` ActionValue))
  ;[1 1 1] Controller：スティック操作
  (:`Triggered`
    (`self.AddControllerYawInput` _x) ; 左スティック：移動操作
    (`self.AddControllerPitchInput` _y) ; 右スティック：カメラ操作
  ))

(event `EnhancedInput|/Game/InGame/AI/Input/Actions/IA_Move`
  (params (ActionValue :type "Vector2D Structure") (ElapsedSeconds :type "Float (double-precision)") (TriggeredSeconds :type "Float (double-precision)") (InputAction :type "InputAction Object Reference" :default "/Game/InGame/AI/Input/Actions/IA_Move.IA_Move"))
  (bind (_x _y) (`KismetMathLibrary.BreakVector2D` ActionValue))
  ;[1 1 1] キーボード移動
  (:`Triggered`
    (`self.AddMovementInput` (`KismetMathLibrary.Cross_VectorVector` (`SceneComponent.GetRightVector` (`self.Camera`)) (`KismetMathLibrary.Vector_Up`)) _y) ; 前後移動
    (`self.AddMovementInput` (`SceneComponent.GetRightVector` (`self.Camera`)) _x) ; 左右移動
  ))

(fn `BeginSprint`
  (returns (Succeed :type Boolean))
  (if (`self.Is Sprinting`)
    (return false) ; 失敗を返す
    (else
      (set `CharacterMovementComponent.MaxWalkSpeed` 200.0 (`self.CharacterMovement`)) ; スプリント速度を設定
      (set `self.Is Sprinting` true) ; スプリント状態になった
      (return true) ; 成功を返す
    )))

(fn `EndSprint`
  (returns (Succeed :type Boolean))
  (if (`self.Is Sprinting`)
    (set `CharacterMovementComponent.MaxWalkSpeed` 75.0 (`self.CharacterMovement`)) ; 通常歩行時の速度を設定
    (set `self.Is Sprinting` false) ; スプリント状態でない
    (return true)
    (else
      (return false) ; 失敗を返す
    )))

(fn `Get Is Sprinting`
  (returns (ReturnValue :type Boolean))
  (return (`self.Is Sprinting`)))

(fn `GetCurrentFloor`
  (returns (Floor :type "Actor Object Reference"))
  (return (`.HitActor` (`GameplayStatics.BreakHitResult` (`.HitResult` (break `FindFloorResult` (`CharacterMovementComponent.CurrentFloor` (`self.CharacterMovement`))))))))

(fn `UserConstructionScript`
  (locals (`Weapon Mesh` :type "StaticMeshComponent Object Reference"))
  ;[1 1 1] 武器アセットを装着
  (`/Engine/EditorBlueprintResources/StandardMacros.IsValid` (`self.WeaponMeshAsset`)
    (:`Is Valid`
      (bind _returnvalue (`AddComponent|NODE_AddStaticMeshComponent-0` :`bManualAttachment` true)) ; 変数が設定されている時のみ追加
      (bind _output_get (set `local.Weapon Mesh` _returnvalue)) ; 結果をローカル変数に保存
      (`StaticMeshComponent.SetStaticMesh` _output_get (`self.WeaponMeshAsset`))
      (`SceneComponent.K2_AttachToComponent` (`local.Weapon Mesh`) (`self.Mesh`) "weapon_r" "SnapToTarget" "SnapToTarget" "SnapToTarget" true) ; 「weapon_r」ソケットに装着
    )))