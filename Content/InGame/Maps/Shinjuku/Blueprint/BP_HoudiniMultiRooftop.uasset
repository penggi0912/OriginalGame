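; BP_HoudiniMultiRooftop builds rooftop static meshes for the Shinjuku map from placement data tables, apparently exported from Houdini.
; The construction script reads each placement row, finds the RooftopList row matching its asset name, and adds a component with that mesh.
; Transforms are converted by swapping Y and Z position, scaling position, adding a per-asset offset, using only negated, offset yaw, and enlarging scale.
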(fn `UserConstructionScript`
  (locals (NewLocalVar_0 :type "HierarchicalInstancedStaticMeshComponent Object Reference") (NewLocalVar_1 :type "HierarchicalInstancedStaticMeshComponent Object Reference") (NewLocalVar_2 :type "Rotator Structure" :default (struct)))
  (bind _scaleposition (`self.ScalePosition`))
  (bind _outrownames (`DataTableFunctionLibrary.GetDataTableRowNames` (`self.datatable`)))
  (for _array_element _outrownames
    (bind _returnvalue (`|GetDataTableRow` (`self.datatable`) _array_element)
      (:`then`
        (bind _outrownames_2 (`DataTableFunctionLibrary.GetDataTableRowNames` (`self.RooftopList`)))
        (for _array_element_2 _outrownames_2
          (bind (_assets _p _scale _cd _rot) (break `/Game/InGame/Maps/Shinjuku/Blueprint/HoudiniRooftopTransform` _returnvalue))
          (if (== _array_element_2 _assets)
            (bind _returnvalue_2 (`|GetDataTableRow` (`self.RooftopList`) _array_element_2)
              (:`then`
                (bind (_mesh _offsetposition) (break `/Game/InGame/Maps/Shinjuku/Blueprint/ArrayRooftop` _returnvalue_2))
                (bind _returnvalue_3 (`AddComponent|NODE_AddStaticMeshComponent-4` :`RelativeTransform` (`KismetMathLibrary.MakeTransform` (+ (`KismetMathLibrary.MakeVector` (* (`|GetArrayItem` _p) _scaleposition) (* (`|GetArrayItem` _p 2) _scaleposition) (* (`|GetArrayItem` _p 1) _scaleposition)) _offsetposition) (`KismetMathLibrary.MakeRotator` 0.0 0.0 (+ (* (`|GetArrayItem` _rot 1) -1.0) 1.0)) (* (100.0 100.0 100.0) (`KismetMathLibrary.MakeVector` (`|GetArrayItem` _scale) (`|GetArrayItem` _scale 1) (`|GetArrayItem` _scale 2))))))
                (`StaticMeshComponent.SetStaticMesh` _returnvalue_3 _mesh)))))))))