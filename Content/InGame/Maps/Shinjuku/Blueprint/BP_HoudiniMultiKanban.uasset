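; Construction-script actor that populates the Shinjuku map with signboards (kanban) from a data table of placements, apparently exported from Houdini.
; MakeTransform swaps Y/Z axes, negates yaw and looks up each asset in KanbanList for mesh, type, offsets and scale range.
; Each sign becomes a static mesh component whose dynamic material gets a wide, square or tall texture by type.
; Texture picks use a random stream, but scale variation is unseeded.
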(fn `MakeTransform`
  (params (DataTable :type "DataTable Object Reference") (RowName :type Name))
  (returns (Location :type "Vector Structure") (ZRotation :type "Float (double-precision)") (Scale :type "Vector Structure") (Mash :type "StaticMesh Object Reference") (Type :type String))
  (bind _scaleposition (`self.ScalePosition`))
  (bind _returnvalue (`|GetDataTableRow` DataTable RowName)
    (:`then`
      (bind _outrownames (`DataTableFunctionLibrary.GetDataTableRowNames` (`self.kanbanList`)))
      (for _array_element _outrownames
        (bind (_assets _p _scale _cd _rot) (break `/Game/InGame/Maps/Shinjuku/Blueprint/HoudiniMultiKanban` _returnvalue))
        (if (== _assets _array_element)
          (bind _returnvalue_2 (`|GetDataTableRow` (`self.kanbanList`) _array_element)
            (:`then`
              (bind (_mesh _scalemin _scalemax _offsetposition _scale_2 _offsetrot _type) (break `/Game/InGame/Maps/Shinjuku/Blueprint/ArrayKanban` _returnvalue_2))
              (return (+ (`KismetMathLibrary.MakeVector` (* (`|GetArrayItem` _p) _scaleposition) (* (`|GetArrayItem` _p 2) _scaleposition) (* (`|GetArrayItem` _p 1) _scaleposition)) _offsetposition) (+ (* (`|GetArrayItem` _rot 1) -1.0) _offsetrot) (* (* (`KismetMathLibrary.Conv_DoubleToVector` (`KismetMathLibrary.RandomFloatInRange` _scalemin _scalemax)) _scale_2) (`KismetMathLibrary.MakeVector` (`|GetArrayItem` _scale) (`|GetArrayItem` _scale 2) (`|GetArrayItem` _scale 1))) _mesh _type))))))
    (:`RowNotFound`
      (return (+ (`KismetMathLibrary.MakeVector` (* (`|GetArrayItem` _p) _scaleposition) (* (`|GetArrayItem` _p 2) _scaleposition) (* (`|GetArrayItem` _p 1) _scaleposition)) _offsetposition) (+ (* (`|GetArrayItem` _rot 1) -1.0) _offsetrot) (* (* (`KismetMathLibrary.Conv_DoubleToVector` (`KismetMathLibrary.RandomFloatInRange` _scalemin _scalemax)) _scale_2) (`KismetMathLibrary.MakeVector` (`|GetArrayItem` _scale) (`|GetArrayItem` _scale 2) (`|GetArrayItem` _scale 1))) _mesh _type))))

(fn `UserConstructionScript`
  (locals (NewLocalVar_0 :type "HierarchicalInstancedStaticMeshComponent Object Reference") (NewLocalVar_1 :type "HierarchicalInstancedStaticMeshComponent Object Reference") (NewLocalVar_2 :type "Rotator Structure" :default (struct)))
  (bind _stream (`self.Stream`))
  (bind _squaretexture (`self.SquareTexture`))
  (bind _squaretexture_2 (`self.SquareTexture`))
  (bind _talltexture (`self.TallTexture`))
  (bind _widetexture (`self.WideTexture`))
  (bind _squaretexture_3 (`self.SquareTexture`))
  (bind _talltexture_2 (`self.TallTexture`))
  (bind _widetexture_2 (`self.WideTexture`))
  (bind _widetexture_3 (`self.WideTexture`))
  (bind _squaretexture_4 (`self.SquareTexture`))
  (bind _squaretexture_5 (`self.SquareTexture`))
  (bind _squaretexture_6 (`self.SquareTexture`))
  (bind _talltexture_3 (`self.TallTexture`))
  (bind _squaretexture_7 (`self.SquareTexture`))
  (bind _talltexture_4 (`self.TallTexture`))
  (bind _widetexture_4 (`self.WideTexture`))
  (bind _outrownames (`DataTableFunctionLibrary.GetDataTableRowNames` (`self.datatable`)))
  (for _array_element _outrownames
    (bind (_location _zrotation _scale _mash _type) (`self.MakeTransform` (`self.datatable`) _array_element))
    (bind _returnvalue (`AddComponent|NODE_AddStaticMeshComponent-2` :`RelativeTransform` (`KismetMathLibrary.MakeTransform` _location (`KismetMathLibrary.MakeRotator` 0.0 0.0 _zrotation) (`KismetMathLibrary.MakeVector` (.y _scale) (.x _scale) (.z _scale)))))
    (`StaticMeshComponent.SetStaticMesh` _returnvalue _mash)
    (bind _returnvalue_2 (`PrimitiveComponent.CreateDynamicMaterialInstance` _returnvalue 0 null "None"))
    (if (== _type "landscape")
      (`MaterialInstanceDynamic.SetTextureParameterValue` _returnvalue_2 "Texture" (`|GetArrayItem` _widetexture_3 (`KismetMathLibrary.RandomIntegerFromStream` _stream (`KismetArrayLibrary.Array_Length` _widetexture_3))))
      (elif (== _type "square")
        (`MaterialInstanceDynamic.SetTextureParameterValue` _returnvalue_2 "Texture" (`|GetArrayItem` _squaretexture (`KismetMathLibrary.RandomIntegerFromStream` _stream (`KismetArrayLibrary.Array_Length` _squaretexture))))
        (elif (== _type "poster")
          (`MaterialInstanceDynamic.SetTextureParameterValue` _returnvalue_2 "Texture" (`|GetArrayItem` _squaretexture_4 (`KismetMathLibrary.RandomIntegerFromStream` _stream (`KismetArrayLibrary.Array_Length` _squaretexture_4))))
          (elif (== _type "standsign")
            (`MaterialInstanceDynamic.SetTextureParameterValue` _returnvalue_2 "Texture" (`|GetArrayItem` _squaretexture_5 (`KismetMathLibrary.RandomIntegerFromStream` _stream (`KismetArrayLibrary.Array_Length` _squaretexture_5))))
            (elif (== _type "entrancesign")
              (`MaterialInstanceDynamic.SetTextureParameterValue` _returnvalue_2 "Texture" (`|GetArrayItem` _squaretexture_6 (`KismetMathLibrary.RandomIntegerFromStream` _stream (`KismetArrayLibrary.Array_Length` _squaretexture_6))))
              (elif (== _type "vertical")
                (`MaterialInstanceDynamic.SetTextureParameterValue` _returnvalue_2 "Texture" (`|GetArrayItem` _talltexture_3 (`KismetMathLibrary.RandomIntegerFromStream` _stream (`KismetArrayLibrary.Array_Length` _talltexture_3))))
                (elif (== _type "Square")
                  (`MaterialInstanceDynamic.SetTextureParameterValue` _returnvalue_2 "Texture" (`|GetArrayItem` _squaretexture_7 (`KismetMathLibrary.RandomIntegerFromStream` _stream (`KismetArrayLibrary.Array_Length` _squaretexture_7))))
                  (elif (== _type "Tall")
                    (`MaterialInstanceDynamic.SetTextureParameterValue` _returnvalue_2 "Texture" (`|GetArrayItem` _talltexture_4 (`KismetMathLibrary.RandomIntegerFromStream` _stream (`KismetArrayLibrary.Array_Length` _talltexture_4))))
                    (elif (== _type "Wide")
                      (`MaterialInstanceDynamic.SetTextureParameterValue` _returnvalue_2 "Texture" (`|GetArrayItem` _widetexture_4 (`KismetMathLibrary.RandomIntegerFromStream` _stream (`KismetArrayLibrary.Array_Length` _widetexture_4))))
                      (elif (== _type "Square_Back")
                        (`MaterialInstanceDynamic.SetTextureParameterValue` _returnvalue_2 "Texture" (`|GetArrayItem` _squaretexture_2 (`KismetMathLibrary.RandomIntegerFromStream` _stream (`KismetArrayLibrary.Array_Length` _squaretexture_2))))
                        (elif (== _type "Tall_Back")
                          (`MaterialInstanceDynamic.SetTextureParameterValue` _returnvalue_2 "Texture" (`|GetArrayItem` _talltexture (`KismetMathLibrary.RandomIntegerFromStream` _stream (`KismetArrayLibrary.Array_Length` _talltexture))))
                          (elif (== _type "Wide_Back")
                            (`MaterialInstanceDynamic.SetTextureParameterValue` _returnvalue_2 "Texture" (`|GetArrayItem` _widetexture (`KismetMathLibrary.RandomIntegerFromStream` _stream (`KismetArrayLibrary.Array_Length` _widetexture))))
                            (elif (== _type "SquareBox")
                              (`MaterialInstanceDynamic.SetTextureParameterValue` _returnvalue_2 "Texture" (`|GetArrayItem` _squaretexture_3 (`KismetMathLibrary.RandomIntegerFromStream` _stream (`KismetArrayLibrary.Array_Length` _squaretexture_3))))
                              (elif (== _type "S_Tall")
                                (`MaterialInstanceDynamic.SetTextureParameterValue` _returnvalue_2 "Texture" (`|GetArrayItem` _talltexture_2 (`KismetMathLibrary.RandomIntegerFromStream` _stream (`KismetArrayLibrary.Array_Length` _talltexture_2))))
                                (elif (== _type "S_Wide")
                                  (`MaterialInstanceDynamic.SetTextureParameterValue` _returnvalue_2 "Texture" (`|GetArrayItem` _widetexture_2 (`KismetMathLibrary.RandomIntegerFromStream` _stream (`KismetArrayLibrary.Array_Length` _widetexture_2)))))))))))))))))))))