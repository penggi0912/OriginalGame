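; Construction-script placer for the Shinjuku map that dresses the level from Houdini-exported point data.
; Each point row is matched by name to an AssetList row, converting position to Unreal axes and centimetres, then spawning a decal or static mesh component.
; A random stream varies scale, yaw and sign, bicycle, bin and vending machine variants.
; Trees gain pots, hedges use point scale, and cargo van variants have empty mesh slots.
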(fn `UserConstructionScript`
  (locals (NewLocalVar_0 :type "HierarchicalInstancedStaticMeshComponent Object Reference") (NewLocalVar_1 :type "HierarchicalInstancedStaticMeshComponent Object Reference") (NewLocalVar_2 :type "Rotator Structure" :default (struct)))
  (bind _outrownames (`DataTableFunctionLibrary.GetDataTableRowNames` (`self.datatable`)))
  (for _array_element _outrownames
    (bind _returnvalue (`|GetDataTableRow` (`self.datatable`) _array_element)
      (:`then`
        (bind _outrownames_2 (`DataTableFunctionLibrary.GetDataTableRowNames` (`self.AssetList`)))
        (for _array_element_2 _outrownames_2
          (bind (_assets _p _scale _cd _rot) (break `/Game/InGame/Maps/Shinjuku/Blueprint/HoudiniMultiTransform` _returnvalue))
          (if (== _assets _array_element_2)
            (bind _returnvalue_2 (`|GetDataTableRow` (`self.AssetList`) _array_element_2)
              (:`then`
                (bind (_mesh _decal _scalemin _scalemax _decalmode _randomrot _offsetposition _scale_2 _offsetrot) (break `/Game/InGame/Maps/Shinjuku/Blueprint/ArrayActor` _returnvalue_2))
                (if _decalmode
                  (bind _returnvalue_3 (`KismetMathLibrary.MakeVector` (* (`|GetArrayItem` _p) 100.0) (* (`|GetArrayItem` _p 2) 100.0) (* (`|GetArrayItem` _p 1) 100.0)))
                  (bind _returnvalue_4 (+ (* (`|GetArrayItem` _rot 1) -1.0) _offsetrot))
                  (bind _output (`|GetArrayItem` _scale 2))
                  ;[1 1 1] decal
                  (bind _returnvalue_5 (`AddComponent|NODE_AddDecalComponent-0` :`RelativeTransform` (`KismetMathLibrary.MakeTransform` _returnvalue_3 (`KismetMathLibrary.MakeRotator` 0.0 -90.0 _returnvalue_4) (`KismetMathLibrary.MakeVector` (`|GetArrayItem` _scale 1) _output (`|GetArrayItem` _scale)))))
                  (`DecalComponent.SetDecalMaterial` _returnvalue_5 _decal)
                  (bind _returnvalue_6 (`DecalComponent.CreateDynamicMaterialInstance` _returnvalue_5))
                  (`MaterialInstanceDynamic.SetScalarParameterValue` _returnvalue_6 "Scale" (/ _output 2.0))
                  (elif _randomrot
                    (bind _returnvalue_7 (* (`KismetMathLibrary.Conv_DoubleToVector` (`KismetMathLibrary.RandomFloatInRangeFromStream` (`self.Stream`) _scalemin _scalemax)) _scale_2))
                    (bind _returnvalue_8 (`AddComponent|NODE_AddStaticMeshComponent-0` :`RelativeTransform` (`KismetMathLibrary.MakeTransform` _returnvalue_3 (`KismetMathLibrary.MakeRotator` 0.0 0.0 (`KismetMathLibrary.RandomFloatInRangeFromStream` (`self.Stream`) 0.0 360.0)) _returnvalue_7)))
                    (`SceneComponent.K2_AddLocalOffset` _returnvalue_8 _offsetposition false false)
                    (`StaticMeshComponent.SetStaticMesh` _returnvalue_8 _mesh)
                    (if (== _mesh (`self.tree`))
                      (bind _returnvalue_9 (`AddComponent|NODE_AddStaticMeshComponent-7` :`RelativeTransform` (`KismetMathLibrary.MakeTransform` (+ _returnvalue_3 (0.0 0.0 -22.0)) (`KismetMathLibrary.MakeRotator` 0.0 0.0 _returnvalue_4) (* (0.02 0.02 0.02) (0.7 0.7 0.2)))))
                      (`StaticMeshComponent.SetStaticMesh` _returnvalue_9 "/Game/Megascans/3D_Assets/Concrete_Plant_Pot_ui1ldhkba/Concrete_Plant_Pot_LOD0_ui1ldhkba.Concrete_Plant_Pot_LOD0_ui1ldhkba"))
                    (elif (== _mesh (`self.Hedge`))
                      ;[1 1 1] Hedge
                      (bind _returnvalue_10 (`AddComponent|NODE_AddStaticMeshComponent-2` :`RelativeTransform` (`KismetMathLibrary.MakeTransform` _returnvalue_3 (`KismetMathLibrary.MakeRotator` 0.0 0.0 _returnvalue_4) (`KismetMathLibrary.MakeVector` (.x (* (`KismetMathLibrary.MakeVector` (`|GetArrayItem` _scale 2) (`|GetArrayItem` _scale) (`|GetArrayItem` _scale 1)) (1.0 0.3 1.0))) (.y (* (`KismetMathLibrary.MakeVector` (`|GetArrayItem` _scale 2) (`|GetArrayItem` _scale) (`|GetArrayItem` _scale 1)) (1.0 0.3 1.0))) (.z (* (`KismetMathLibrary.MakeVector` (`|GetArrayItem` _scale 2) (`|GetArrayItem` _scale) (`|GetArrayItem` _scale 1)) (1.0 0.3 1.0)))))))
                      (`StaticMeshComponent.SetStaticMesh` _returnvalue_10 _mesh)
                      (else
                        (bind _returnvalue_11 (`AddComponent|NODE_AddStaticMeshComponent-3` :`RelativeTransform` (`KismetMathLibrary.MakeTransform` _returnvalue_3 (`KismetMathLibrary.MakeRotator` 0.0 0.0 _returnvalue_4) _returnvalue_7)))
                        (switch `string` (`KismetSystemLibrary.GetDisplayName` _mesh)
                          (:`Default`
                            (`SceneComponent.K2_AddLocalOffset` _returnvalue_11 _offsetposition false false)
                            ;[1 1 1] 車
                            (`StaticMeshComponent.SetStaticMesh` _returnvalue_11 _mesh))
                          (:`SM_CrossingSign00`
                            ;[1 1 1] Sign
                            (switch `int` (`KismetMathLibrary.RandomIntegerInRangeFromStream` (`self.Stream`) 0 6)
                              (:`0`
                                (`StaticMeshComponent.SetStaticMesh` _returnvalue_11 "/Game/Imports/Props/SM_CrossingSign00.SM_CrossingSign00"))
                              (:`1`
                                (`StaticMeshComponent.SetStaticMesh` _returnvalue_11 "/Game/Imports/Props/SM_CyclingSign00.SM_CyclingSign00"))
                              (:`2`
                                (`StaticMeshComponent.SetStaticMesh` _returnvalue_11 "/Game/Imports/Props/SM_FireCisternSign00.SM_FireCisternSign00"))
                              (:`3`
                                (`StaticMeshComponent.SetStaticMesh` _returnvalue_11 "/Game/Imports/Props/SM_NoParkingSign00.SM_NoParkingSign00"))
                              (:`4`
                                (`StaticMeshComponent.SetStaticMesh` _returnvalue_11 "/Game/Imports/Props/SM_PedestriansSign00.SM_PedestriansSign00"))
                              (:`5`
                                (`StaticMeshComponent.SetStaticMesh` _returnvalue_11 "/Game/Imports/Props/SM_SpeedLimitSign00.SM_SpeedLimitSign00"))
                              (:`6`
                                (`StaticMeshComponent.SetStaticMesh` _returnvalue_11 "/Game/Imports/Props/SM_StopSign00.SM_StopSign00"))))
                          (:`SM_Bicycle_01A`
                            ;[1 1 1] 自転車
                            (switch `int` (`KismetMathLibrary.RandomIntegerInRangeFromStream` (`self.Stream`) 0 2)
                              (:`0`
                                (`StaticMeshComponent.SetStaticMesh` _returnvalue_11 "/Game/Imports/Props/SM_Bicycle_01A.SM_Bicycle_01A"))
                              (:`1`
                                (`StaticMeshComponent.SetStaticMesh` _returnvalue_11 "/Game/Imports/Props/SM_Bicycle_01B.SM_Bicycle_01B"))
                              (:`2`
                                (`StaticMeshComponent.SetStaticMesh` _returnvalue_11 "/Game/Imports/Props/SM_Bicycle_01C.SM_Bicycle_01C"))))
                          (:`SM_GarbageCan_01A`
                            ;[1 1 1] 自転車
                            (switch `int` (`KismetMathLibrary.RandomIntegerInRangeFromStream` (`self.Stream`) 0 2)
                              (:`0`
                                (`StaticMeshComponent.SetStaticMesh` _returnvalue_11 "/Game/Imports/Props/SM_GarbageCan_01A.SM_GarbageCan_01A"))
                              (:`1`
                                (`StaticMeshComponent.SetStaticMesh` _returnvalue_11 "/Game/Imports/Props/SM_GarbageCan_01B.SM_GarbageCan_01B"))
                              (:`2`
                                (`StaticMeshComponent.SetStaticMesh` _returnvalue_11 "/Game/Imports/Props/SM_GarbageCan_01C.SM_GarbageCan_01C"))))
                          (:`SM_VendingMachine_01A`
                            ;[1 1 1] 自販機
                            (switch `int` (`KismetMathLibrary.RandomIntegerInRangeFromStream` (`self.Stream`) 0 2)
                              (:`0`
                                (`StaticMeshComponent.SetStaticMesh` _returnvalue_11 "/Game/Imports/Props/SM_VendingMachine_01A.SM_VendingMachine_01A"))
                              (:`1`
                                (`StaticMeshComponent.SetStaticMesh` _returnvalue_11 "/Game/Imports/Props/SM_VendingMachine_01B.SM_VendingMachine_01B"))
                              (:`2`
                                (`StaticMeshComponent.SetStaticMesh` _returnvalue_11 "/Game/Imports/Props/SM_VendingMachine_01C.SM_VendingMachine_01C"))))
                          (:`SM_Cargo_Van_Car`
                            (switch `int` (`KismetMathLibrary.RandomIntegerInRangeFromStream` (`self.Stream`) 0 12)
                              (:`0`
                                (`StaticMeshComponent.SetStaticMesh` _returnvalue_11 null))
                              (:`1`
                                (`StaticMeshComponent.SetStaticMesh` _returnvalue_11 null))
                              (:`2`
                                (`StaticMeshComponent.SetStaticMesh` _returnvalue_11 null))
                              (:`3`
                                (`StaticMeshComponent.SetStaticMesh` _returnvalue_11 null))
                              (:`4`
                                (`StaticMeshComponent.SetStaticMesh` _returnvalue_11 null))
                              (:`5`
                                (`StaticMeshComponent.SetStaticMesh` _returnvalue_11 null))
                              (:`6`
                                (`StaticMeshComponent.SetStaticMesh` _returnvalue_11 null))
                              (:`7`
                                (`StaticMeshComponent.SetStaticMesh` _returnvalue_11 null))
                              (:`8`
                                (`StaticMeshComponent.SetStaticMesh` _returnvalue_11 null))
                              (:`9`
                                (`StaticMeshComponent.SetStaticMesh` _returnvalue_11 null))
                              (:`10`
                                (`StaticMeshComponent.SetStaticMesh` _returnvalue_11 null))
                              (:`11`
                                (`StaticMeshComponent.SetStaticMesh` _returnvalue_11 null))
                              (:`12`
                                (`StaticMeshComponent.SetStaticMesh` _returnvalue_11 null))
                              (:`13`
                                (`StaticMeshComponent.SetStaticMesh` _returnvalue_11 null))))))))))))))))
  (`KismetSystemLibrary.PrintString` (`KismetStringLibrary.Conv_IntToString` 0)))