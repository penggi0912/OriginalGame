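; BP_FuncLibrary is a Blueprint function library of shared gameplay helpers for rays, player-pawn checks, sine waves, items and damage.
; Item loaders map DataTable rows to item fields with zero count; LoadAllItemList returns at the first found row despite its loop.
; Physical and magic damage share one formula: scaled attack plus fixed value minus scaled defense, unclamped.
; ObtainItems is an unfinished stub with disconnected debug nodes.
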(fn CalcRay
  (params (Origin :type Vector) (Direction :type Vector) (Length :type Float%20%28double-precision%29))
  ;[1 1 1] 光線の計算
  (return Origin (+ Origin (* Direction Length))))

(fn IsPlayerPawn
  (params (Actor :type Actor%20Object%20Reference))
  ;[1 1 1] 自機判定
  (bind _aspawn (Utilities|Casting|CastToPawn Actor) ; アクタがポーンかどうかを判定
    (:then
      (Utilities|Casting|CastToPlayerController (Pawn|GetController _aspawn) ; 自機かどうかを判定
        (:then
          (return true))
        (:CastFailed
          _)))
    (:CastFailed
      _))
  (return false))

(fn SineCurve
  (params (Amplitude :type Float%20%28double-precision%29) (Period :type Float%20%28double-precision%29) (Time :type Float%20%28double-precision%29) (Phase :type Float%20%28double-precision%29))
  ;[1 1 1] A sin(2π/T*t+θ)で正弦波を計算
  (return (|(A*(sin(((w*t)+theta)))) Amplitude (Math|Float|SafeDivide (Math|Float|MultiplybyPi 2.0) Period) Time Phase)))

(fn ObtainItems
  (params (Player%20Controller :type BP%20Player%20Controller%20Object%20Reference))
  ;[1 1 1] プレイヤーがアイテムを獲得したら所持数増加
)

(fn LoadAllItemList
  (params (Table :type Data%20Table%20Object%20Reference))
  (bind _outrownames (DataTable|GetDataTableRowNames Table))
  (for _array_element _outrownames
    (bind _returnvalue (Utilities|GetDataTableRow Table _array_element)
      (:then
        (return (.EN_ItemCategory (Utilities|Struct|BreakST_ItemData _returnvalue)) (.EN_ItemRarity (Utilities|Struct|BreakST_ItemData _returnvalue)) (.ItemName (Utilities|Struct|BreakST_ItemData _returnvalue)) (.ItemDesc (Utilities|Struct|BreakST_ItemData _returnvalue)) (.Image (Utilities|Struct|BreakST_ItemData _returnvalue)) 0 (.MaxQuantity (Utilities|Struct|BreakST_ItemData _returnvalue)) (.Value (Utilities|Struct|BreakST_ItemData _returnvalue)) (.BuyPrice (Utilities|Struct|BreakST_ItemData _returnvalue)) (.SalePrice (Utilities|Struct|BreakST_ItemData _returnvalue)) (.Stackable (Utilities|Struct|BreakST_ItemData _returnvalue)) (.ItemClass (Utilities|Struct|BreakST_ItemData _returnvalue)))))))

(fn LoadItemList
  (params (DataTable :type Data%20Table%20Object%20Reference) (RowName :type Name))
  (bind _returnvalue (Utilities|GetDataTableRow DataTable RowName)
    (:then
      (return (.EN_ItemCategory (Utilities|Struct|BreakST_ItemData _returnvalue)) (.EN_ItemRarity (Utilities|Struct|BreakST_ItemData _returnvalue)) (.ItemName (Utilities|Struct|BreakST_ItemData _returnvalue)) (.ItemDesc (Utilities|Struct|BreakST_ItemData _returnvalue)) (.Image (Utilities|Struct|BreakST_ItemData _returnvalue)) 0 (.MaxQuantity (Utilities|Struct|BreakST_ItemData _returnvalue)) (.Value (Utilities|Struct|BreakST_ItemData _returnvalue)) (.BuyPrice (Utilities|Struct|BreakST_ItemData _returnvalue)) (.SalePrice (Utilities|Struct|BreakST_ItemData _returnvalue)) (.Stackable (Utilities|Struct|BreakST_ItemData _returnvalue)) (.ItemClass (Utilities|Struct|BreakST_ItemData _returnvalue))))))

(fn PDamageSystem
  (params (Weapon%20ATK :type Float%20%28double-precision%29) (P_ATK :type Float%20%28double-precision%29) (ATK%20Coefficient :type Float%20%28double-precision%29) (ATK%20Multiplier :type Float%20%28double-precision%29) (ATK%20Fix%20Value :type Float%20%28double-precision%29) (P_DEF :type Float%20%28double-precision%29) (Equip%20DEF :type Float%20%28double-precision%29) (DEFCoefficient :type Float%20%28double-precision%29) (Skill%20DEF%20Multiplier :type Float%20%28double-precision%29))
  ;[1 1 1] 物理ダメージ計算式
  ; ((((攻撃力+武器攻撃力)*攻撃力係数*スキル倍率)+スキル固定値) - ((防御力+装備防御力)*防御力係数*スキル防御倍率) )
  (return (- (+ (* (* (+ Weapon%20ATK P_ATK) ATK%20Coefficient) ATK%20Multiplier) ATK%20Fix%20Value) (* (* (+ P_DEF Equip%20DEF) DEFCoefficient) Skill%20DEF%20Multiplier))))

(fn MDamageSystem
  (params (Weapon%20ATK :type Float%20%28double-precision%29) (M_ATK :type Float%20%28double-precision%29) (ATK%20Coefficient :type Float%20%28double-precision%29) (ATK%20Multiplier :type Float%20%28double-precision%29) (ATK%20Fix%20Value :type Float%20%28double-precision%29) (M_DEF :type Float%20%28double-precision%29) (Equip%20DEF :type Float%20%28double-precision%29) (DEFCoefficient :type Float%20%28double-precision%29) (Skill%20DEF%20Multiplier :type Float%20%28double-precision%29))
  ;[1 1 1] 物理ダメージ計算式
  ; ((((攻撃力+武器攻撃力)*攻撃力係数*スキル倍率)+スキル固定値) - ((防御力+装備防御力)*防御力係数*スキル防御倍率) )
  (return (- (+ (* (* (+ Weapon%20ATK M_ATK) ATK%20Coefficient) ATK%20Multiplier) ATK%20Fix%20Value) (* (* (+ M_DEF Equip%20DEF) DEFCoefficient) Skill%20DEF%20Multiplier))))