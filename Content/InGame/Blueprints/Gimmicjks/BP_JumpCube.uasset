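; BP_JumpCube is a gimmick cube that a pawn standing on it toggles between moving toward DestTransform and back by jumping.
; Stepping on or off swaps the cube's material and binds or unbinds Toggle to BP_PawnSample's jump event.
; A FlipFlop plays or reverses a timeline, which applies per-update delta transforms to the actor, using DummyCube as the previous offset.
; Reset re-triggers the FlipFlop based on its state.
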(event `/Game/InGame/Blueprints/Interfaces/BI_Floor.OnPawnOn`
  (params (Pawn :type "Pawn Object Reference"))
  ;[1 1 1] キューブの上に乗るとスイッチオン
  (`PrimitiveComponent.SetMaterial` (`self.Cube`) 0 "/Game/DragMe/GridMaterials/MI_Grid_G.MI_Grid_G")
  (bind _asbp_pawn_sample (cast `/Game/Imports/PaperNinja/BP_PawnSample` Pawn))
  (add `/Game/Imports/PaperNinja/BP_PawnSample.OnPawnJumped` _asbp_pawn_sample (delegate `Toggle`)))

(event `Toggle`
  ;[1 1 1] キューブの上に乗るとスイッチオン
  ;[1 1 1] リセット動作
  (bind _isa (`/Engine/EditorBlueprintResources/StandardMacros.FlipFlop` :!label _label)
    (:`A`
      ;[1 1 1] キューブ上でジャンプするとキューブ上昇・下降
      (bind (_direction _alpha) (`Timeline|CubeTL` :!label _label_2)
        (:`Update`
          (bind _returnvalue (`KismetMathLibrary.TLerp` (`self.Identity`) (`self.DestTransform`) _alpha))
          (`self.K2_SetActorTransform` (`KismetMathLibrary.ComposeTransforms` (`KismetMathLibrary.ComposeTransforms` _returnvalue (`KismetMathLibrary.InvertTransform` (`self.DummyCube`))) (`self.GetTransform`)))
          (set `self.DummyCube` _returnvalue))))
    (:`B`
      (goto _label_2 :!via `Reverse`))))

(event `Reset`
  ;[1 1 1] リセット動作
  (if (stale `Toggle` _isa)
    (goto _label)))

(event `/Game/InGame/Blueprints/Interfaces/BI_Floor.OnPawnOff`
  (params (Pawn :type "Pawn Object Reference"))
  ;[1 1 1] キューブから離れるとスイッチオフ
  (`PrimitiveComponent.SetMaterial` (`self.Cube`) 0 "/Game/DragMe/GridMaterials/MI_Grid_Y.MI_Grid_Y")
  (bind _asbp_pawn_sample (cast `/Game/Imports/PaperNinja/BP_PawnSample` Pawn))
  (remove `/Game/Imports/PaperNinja/BP_PawnSample.OnPawnJumped` _asbp_pawn_sample (delegate `Toggle`)))

(fn `UserConstructionScript`)