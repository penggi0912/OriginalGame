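; BI_Enemy is a Blueprint interface that defines the functions other objects use to communicate with enemies.
; It exposes getters and setters for the enemy reference, weapon reference and skill motion type, plus getters for status and HP/MP.
; It also declares a shield-hit notification and queries for the projectile attack flag and damage state.
; The functions hold no logic, only default returns, leaving behavior to implementing classes.
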(fn `CheckHaveDamagedEnemy`
  (returns (`HaveDamaged?` :type Boolean))
  (return false))

(fn `GetEnemyHP&MP`
  (returns (MaxHP :type "Float (double-precision)") (CurrentHP :type "Float (double-precision)") (MaxMP :type "Float (double-precision)") (CurrentMP :type "Float (double-precision)"))
  (return 0.0 0.0 0.0 0.0))

(fn `GetEnemyRef`
  (returns (EnemyRef :type "/Game/InGame/Blueprints/Pawns/Enemies/BP_EnemyBase Object Reference"))
  (return null))

(fn `GetEnemySkillMotionType`
  (returns (`Skill Motion Type` :type "/Game/InGame/Blueprints/Data/Enum/EN_EnemySkillMotionType Enum"))
  (return "NewEnumerator9"))

(fn `GetEnemyStatus`
  (returns (EnemyData :type "/Game/InGame/Blueprints/Data/Enemy/ST_EnemyData Structure"))
  (return))

(fn `GetEnemyWeaponRef`
  (returns (EnemyWeaponRef :type "/Game/InGame/Blueprints/Equipment/BP_WeaponBase_Enemy Object Reference"))
  (return null))

(fn `GetProjectileAttackFlg`
  (returns (`IsProjectileAttack?` :type Boolean))
  (return false))

(fn `SetEnemyRef`
  (params (EnemyRef :type "/Game/InGame/Blueprints/Pawns/Enemies/BP_EnemyBase Object Reference")))

(fn `SetEnemySkillMotionType`
  (params (`Skill Motion Type` :type "/Game/InGame/Blueprints/Data/Enum/EN_EnemySkillMotionType Enum" :default "NewEnumerator9")))

(fn `SetEnemyWeaponRef`
  (params (EnemyWeaponRef :type "/Game/InGame/Blueprints/Equipment/BP_WeaponBase_Enemy Object Reference")))

(fn `ShieldHittedEnemy`
  (params (`Is Shield Hitted Enemy` :type Boolean)))