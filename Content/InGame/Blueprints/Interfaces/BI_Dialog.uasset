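; BI_Dialog is a Blueprint interface that defines the contract for in-game dialog objects.
; Implementers supply the current and next dialog IDs, current speaker and choice list, and report whether the dialog auto-advances, can fast-forward or can be skipped.
; They also receive callbacks for dialog start, dialog end, skipping and choice selection by index and text.
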(fn `CanFastForward`
  (returns (CanFastForward :type Boolean))
  (return false))

(fn `CanSkip`
  (returns (IsSkippable :type Boolean))
  (return false))

(fn `GetChoiceList`
  (returns (ChoiceArray :type "Array of Text"))
  (return))

(fn `GetCurrentSpeaker`
  (returns (SpeakerInfo :type "/Game/InGame/Blueprints/Data/Dialog/ST_SpeakerInfo Structure"))
  (return))

(fn `GetDialogID`
  (returns (DialogID :type Name))
  (return "None"))

(fn `GetNextDialogID`
  (returns (NextDialogID :type Name))
  (return "None"))

(fn `IsAutoAdvance`
  (returns (IsAutoAdvance :type Boolean))
  (return false))

(fn `OnChoiceSelected`
  (params (ChoiceIndex :type Integer) (ChoiceText :type Text)))

(fn `OnDialogEnd`)

(fn `OnDialogStart`)

(fn `OnSkipped`)