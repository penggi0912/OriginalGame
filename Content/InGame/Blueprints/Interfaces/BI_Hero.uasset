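; BI_Hero is a Blueprint Interface that declares the contract for exchanging hero state with other game objects.
; Setters pass in the hero Blueprint reference, hero data, weapon reference, enemy skill motion type and shield activation.
; Getters return those hero references and data, plus HP and MP, attacking skill name and item-use data.
; Two checks report invincibility and whether damage has been taken.
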(fn `Check Invinsible`
  (returns (`IsInvinsible?` :type Boolean))
  (return false))

(fn `CheckHaveDamaged`
  (returns (`HaveDamaged?` :type Boolean))
  (return false))

(fn `Get Attacking Skill Name`
  (returns (SkillName :type Name))
  (return "None"))

(fn `Get Hero Data`
  (returns (`Hero Data` :type "/Game/InGame/Blueprints/Data/Player/ST_HeroData Structure"))
  (return))

(fn `Get Hero HP&MP`
  (returns (MaxHP :type "Float (double-precision)") (CurrentHP :type "Float (double-precision)") (MaxMP :type "Float (double-precision)") (CurrentMP :type "Float (double-precision)"))
  (return 0.0 0.0 0.0 0.0))

(fn `Get Hero Ref`
  (returns (`Hero BP Ref` :type "/Game/InGame/Blueprints/Pawns/Characters/BP_HeroBase Object Reference"))
  (return null))

(fn `Get Hero Weapon Ref`
  (returns (`Hero Weapon Ref` :type "/Game/InGame/Blueprints/Equipment/BP_WeaponBase_Hero Object Reference"))
  (return null))

(fn `Get Use Item Data`
  (returns (`Item Data` :type "/Game/InGame/Blueprints/Data/ST_ItemData Structure"))
  (return))

(fn `Set Hero BP Ref`
  (params (`Hero BP Ref` :type "/Game/InGame/Blueprints/Pawns/Characters/BP_HeroBase Object Reference")))

(fn `Set Hero Data`
  (params (HeroData :type "/Game/InGame/Blueprints/Data/Player/ST_HeroData Structure")))

(fn `Set Hero Weapon Ref`
  (params (`Weapon Ref` :type "/Game/InGame/Blueprints/Equipment/BP_WeaponBase_Hero Object Reference")))

(fn `SetEnemiesSkillMotionType`
  (params (SkillMotionType :type "/Game/InGame/Blueprints/Data/Enum/EN_EnemySkillMotionType Enum" :default "NewEnumerator9")))

(fn `SetShieldActivation_2`
  (params (`DoesShieldActivate?` :type Boolean)))