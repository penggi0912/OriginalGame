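; Blueprint interface for items that act as shortcuts, giving callers a common way to display and trigger them.
; It declares queries for icon, name, enabled state, hold requirement and cooldown presence and ratio, plus a hook for when the shortcut is used.
; It holds no logic of its own, so implementing assets supply the behavior.
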(fn `GetCooltimeRatio`
  (returns (CooltimeRatio :type "Float (double-precision)"))
  (return 0.0))

(fn `GetShortcutIcon`
  (returns (Icon :type "Texture2D Object Reference"))
  (return null))

(fn `GetShortcutName`
  (returns (Name :type Text) (Text :type Text))
  (return "" ""))

(fn `HasCooltime`
  (returns (HasCooldown :type Boolean))
  (return false))

(fn `IsEnabled`
  (returns (IsEnabled :type Boolean))
  (return false))

(fn `IsHoldRequired`
  (returns (IsHoldRequired :type Boolean))
  (return false))

(fn `OnShortcutUsed`)