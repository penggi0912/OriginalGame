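; HP-healing pickup item Blueprint that restores the player hero's health when UseItemHeal_HP runs with item data.
; It fetches the hero's HP and data struct through message calls on the player character, then adds the item's Value to CurrentHP.
; If the sum reaches MaxHP, it instead writes MaxHP % CurrentHP, commented as trimming overflow.
; The updated struct goes to the hero's HP bar widget; Interact is empty.
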(event `UseItemHeal_HP`
  (params (`Item Data` :type "/Game/InGame/Blueprints/Data/Item/ST_ItemData Structure"))
  (bind _herodata (`self.HeroData`))
  (bind _herohp_bar_ref (`/Game/InGame/Blueprints/Pawns/Characters/BP_HeroBase.HeroHP_Bar_ref` (`self.HeroBPRef`)))
  ;[1 1 1] アイテム使用効果反映
  (bind _heroref (message `/Game/InGame/Blueprints/Interfaces/BI_Hero.GetHeroRef` (`GameplayStatics.GetPlayerCharacter` 0)))
  (bind _output_get (set `self.HeroBPRef` _heroref))
  (bind (_maxhp _currenthp) (message `/Game/InGame/Blueprints/Interfaces/BI_Hero.GetHeroHP&MP` _output_get))
  (bind _output_get_2 (set `self.MaxHP` _maxhp))
  (bind _output_get_3 (set `self.CurrentHP` _currenthp))
  (bind _herodata_2 (message `/Game/InGame/Blueprints/Interfaces/BI_Hero.GetHeroData` _output_get))
  (set `self.HeroData` _herodata_2)
  (bind _returnvalue (+ _output_get_3 (`.Value_52_64CD8404488C4377BB9F8D8175CB4377` (break `/Game/InGame/Blueprints/Data/Item/ST_ItemData` `Item Data`))))
  (if (>= _returnvalue _output_get_2)
    (bind _structout (setmembers `/Game/InGame/Blueprints/Data/Player/ST_HeroData` :`StructRef` _herodata :`CurrentHP` (mod (`self.MaxHP`) (`self.CurrentHP`)))) ; 余剰を除いたHPをステータスに適用
    (`/Game/InGame/Blueprints/Widget/WBP_HeroHP_Bar.Update HP Bar Heal` _herohp_bar_ref _structout) ; 回復後のHPの値をHPバーウィジェットに送る
    (else
      (bind _structout_2 (setmembers `/Game/InGame/Blueprints/Data/Player/ST_HeroData` :`StructRef` _herodata :`CurrentHP` _returnvalue)) ; 回復後のHPをステータスに適用
      (`/Game/InGame/Blueprints/Widget/WBP_HeroHP_Bar.Update HP Bar Heal` _herohp_bar_ref _structout_2) ; 回復後のHPの値をHPバーウィジェットに送る
    )))

(event `self.Interact`)

(fn `UserConstructionScript`)