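; Base class for pickups that the player obtains by overlapping a sphere.
; A player overlap passing CanBeObtained (pawn lifespan is zero) runs Obtainedlmpl, an empty hook for child classes, then calls OnObtained.
; The actor then destroys itself, unless the hero's inventory widget flags QuantityFull, in which case it clears the flag and stays.
; The remaining hero, item and combat functions are mostly stubs returning empty or default values.
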(event `self.Sphere.OnComponentBeginOverlap`
  (params (OverlappedComponent :type "PrimitiveComponent Object Reference") (OtherActor :type "Actor Object Reference") (OtherComp :type "PrimitiveComponent Object Reference") (OtherBodyIndex :type Integer) (bFromSweep :type Boolean) (SweepResult :type "HitResult Structure (by ref)"))
  ;[1 1 1] 自機判定
  (bind (_aspawn _asplayer_controller) (`/Game/InGame/Blueprints/Libraries/BP_ObjectMacroLibrary.DoIfPlayer` OtherActor))
  (if (`self.CanBeObtained` _aspawn _asplayer_controller)
    ;[1 1 1] 獲得処理
    (`self.Obtainedlmpl` _aspawn)
    (`self.OnObtained`)
    (bind _asbp_hero_base (cast `/Game/InGame/Blueprints/Pawns/Characters/BP_HeroBase` (`GameplayStatics.GetPlayerCharacter` 0)))
    (bind _wbp_iteminventory_test (`/Game/InGame/Blueprints/Pawns/Characters/BP_HeroBase.WBP_ItemInventory_Test` _asbp_hero_base))
    (if (`/Game/InGame/Blueprints/Widget/ItemInventory/WBP_MenuView_Inventory.QuantityFull` _wbp_iteminventory_test)
      (set `/Game/InGame/Blueprints/Widget/ItemInventory/WBP_MenuView_Inventory.QuantityFull` false _wbp_iteminventory_test)
      (else
        (`self.K2_DestroyActor`)))))

(event `Obtainedlmpl`
  (params (Pawn :type "Pawn Object Reference") (PlayerController :type "PlayerController Object Reference"))
  ;[1 1 1] 獲得された時の処理（プレースホルダ）
)

(event `/Game/InGame/Blueprints/Interfaces/BI_Interact.hasInteracted`)

(event `Use Item Data_1`
  (params (ItemData :type "/Game/InGame/Blueprints/Data/ST_ItemData Structure")))

(fn `CanBeObtained`
  (params (Pawn :type "Pawn Object Reference") (PlayerController :type "PlayerController Object Reference"))
  (returns (ReturnValue :type Boolean))
  (return (== (`self.GetLifeSpan` Pawn) 0.0)))

(fn `CheckHasDamaged`
  (returns (`hasDamaged?` :type Boolean))
  (return false))

(fn `CheckInvinsible`
  (returns (`isInvinsible?` :type Boolean))
  (return false))

(fn `Get Item Data`
  (returns (`Item Data` :type "/Game/InGame/Blueprints/Data/ST_ItemData Structure"))
  (return (`self.Item Data`)))

(fn `GetAttackingSkillName`
  (returns (skillName :type Name))
  (return "None"))

(fn `GetHeroData`
  (returns (heroData :type "/Game/InGame/Blueprints/Data/Player/ST_HeroData Structure"))
  (return))

(fn `GetHeroHP&MP`
  (returns (maxHP :type "Float (double-precision)") (currentHP :type "Float (double-precision)") (maxMP :type "Float (double-precision)") (currentMP :type "Float (double-precision)"))
  (return 0.0 0.0 0.0 0.0))

(fn `GetHeroRef`
  (returns (heroRef :type "/Game/InGame/Blueprints/Pawns/Characters/BP_HeroBase Object Reference"))
  (return null))

(fn `GetHeroWeaponRef`
  (returns (heroWeaponRef :type "/Game/InGame/Blueprints/Equipment/BP_WeaponBase_Hero Object Reference"))
  (return null))

(fn `getItemData`
  (returns (ItemData :type "/Game/InGame/Blueprints/Data/ST_ItemData Structure"))
  (return))

(fn `GetUseItemData`
  (returns (itemData :type "/Game/InGame/Blueprints/Data/ST_ItemData Structure"))
  (return))

(fn `UserConstructionScript`)