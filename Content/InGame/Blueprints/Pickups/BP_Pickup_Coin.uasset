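; Coin pickup that adds one to Money on the player state when obtained and prints a debug count.
; When spawned as Tossed, it ignores Pawn overlaps for the first second and flies under gravity, integrated manually in Tick with a swept offset.
; On a blocking hit it reflects velocity, keeping only a damped vertical component, and stops simulating once speed falls below SleepThreshold.
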(event `self.ReceiveBeginPlay`
  ;[1 1 1] コイントス開始時、1秒間のみポーンへのコリジョン無視
  (if (`self.Tossed`)
    (`PrimitiveComponent.SetCollisionResponseToChannel` (`self.Trigger`) "ECC_Pawn" "ECR_Ignore")
    (`KismetSystemLibrary.Delay` 1.0)
    (`PrimitiveComponent.SetCollisionResponseToChannel` (`self.Trigger`) "ECC_Pawn" "ECR_Overlap")))

(event `self.ReceiveTick`
  (params (DeltaSeconds :type "Float (single-precision)"))
  ;[1 1 1] ボーナスコインのスポーンの仕方（トス運動）
  (if (`self.Tossed`)
    ;;[1 1 1] 速度の更新
    (set `self.Toss Velocity` (+ (`self.Toss Velocity`) (* (`self.Grabity`) DeltaSeconds)))
    (bind _sweephitresult (`self.K2_AddActorWorldOffset` (* (`self.Toss Velocity`) DeltaSeconds) true))
    (bind (_bblockinghit _binitialoverlap _time _distance _location _impactpoint _normal) (`GameplayStatics.BreakHitResult` _sweephitresult))
    ;;[1 1 1] コインの反射処理
    (if _bblockinghit
      (bind _output_get (set `self.Toss Velocity` (* (`KismetMathLibrary.GetReflectionVector` (`self.Toss Velocity`) _normal) (0.0 0.0 0.8))))
      ;;[1 1 1] 速度が指定値より小さくなったら運動の計算停止
      (if (< (`KismetMathLibrary.VSize` _output_get) (`self.SleepThreshold`))
        (set `self.Tossed` false)))))

(event `self.Obtainedlmpl`
  (params (Pawn :type "Pawn Object Reference") (PlayerController :type "PlayerController Object Reference"))
  ;[1 1 1] プレイヤーがコインを獲得したら獲得枚数増加
  (bind _asbp_player_state (cast `/Game/InGame/Blueprints/System/BP_PlayerState` (`Controller.PlayerState` PlayerController)))
  (bind _result (`/Engine/EditorBlueprintResources/StandardMacros.IncrementInt` (`/Game/InGame/Blueprints/System/BP_PlayerState.Money` _asbp_player_state))
    (:`  `
      (`KismetSystemLibrary.PrintString` (`KismetStringLibrary.Concat_StrStr` "コインの枚数=" (`KismetStringLibrary.Conv_IntToString` _result))))))

(fn `UserConstructionScript`)