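; BP_HPHealItem is a pickup item that restores the player hero's HP when used.
; UseItemHPHeal adds the item's Value to BP_HeroBase's PlayerData HP.
; When the sum reaches MaxHP, it uses MaxHP modulo the sum, which caps overflow at MaxHP but yields zero on an exact match.
; The updated struct feeds the hero HP bar's heal update, while Interact is empty.
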(event `Use Item HPHeal`
  (params (`Item Data` :type "/Game/InGame/Blueprints/Data/ST_ItemData Structure"))
  ;[1 1 1] アイテム使用効果反映
  (bind _asbp_hero_base (cast `/Game/InGame/Blueprints/Pawns/Characters/BP_HeroBase` (`GameplayStatics.GetPlayerCharacter` 0)))
  (bind (_transform _stagelevel _name _characterlevel _totalexp _preexp _maxhp _hp) (break `/Game/InGame/Blueprints/Data/Player/ST_PlayerData` (`/Game/InGame/Blueprints/Pawns/Characters/BP_HeroBase.Player Data` _asbp_hero_base)))
  (bind _returnvalue (+ _hp (`.Value_52_64CD8404488C4377BB9F8D8175CB4377` (break `/Game/InGame/Blueprints/Data/ST_ItemData` `Item Data`))))
  (if (>= _returnvalue _maxhp)
    (bind _player_data (`/Game/InGame/Blueprints/Pawns/Characters/BP_HeroBase.Player Data` _asbp_hero_base))
    (bind _structout (setmembers `/Game/InGame/Blueprints/Data/Player/ST_PlayerData` :`StructRef` _player_data :`HP` (mod _maxhp _returnvalue))) ; 余剰を除いてHPに適用
    (bind _herohp_bar_ref (`/Game/InGame/Blueprints/Pawns/Characters/BP_HeroBase.HeroHP_Bar_ref` _asbp_hero_base))
    (`/Game/InGame/Blueprints/Widget/WBP_HeroHP_Bar.Update HP Bar Heal` _herohp_bar_ref _structout)
    (else
      (bind _structout_2 (setmembers `/Game/InGame/Blueprints/Data/Player/ST_PlayerData` :`StructRef` _player_data :`HP` _returnvalue)) ; HPに適用
      (`/Game/InGame/Blueprints/Widget/WBP_HeroHP_Bar.Update HP Bar Heal` _herohp_bar_ref _structout_2))))

(event `self.Interact`)

(fn `UserConstructionScript`)