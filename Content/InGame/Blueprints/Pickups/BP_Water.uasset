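; BP_Water is the water item pickup, which goes into the hero's inventory when obtained.
; Tick looks up the "Water" row in DT_ItemData every frame and stores it in ItemInfo.
; The Obtainedlmpl event casts the pawn to BP_Hero and passes ItemInfo to AddToInventory on its WBPItemInventoryTest widget.
; BeginPlay and overlap events are disabled placeholders.
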(event `self.ReceiveTick`
  (params (DeltaSeconds :type "Float (single-precision)"))
  ;[1 1 1] アイテムデータセット
  (bind _returnvalue (`|GetDataTableRow` "/Game/InGame/Blueprints/Data/DT_ItemData.DT_ItemData" "Water")
    (:`then`
      (set `self.ItemInfo` _returnvalue))))

(event `/Game/InGame/Blueprints/Pickups/BP_Pickup.Obtainedlmpl`
  (params (Pawn :type "Pawn Object Reference") (PlayerController :type "PlayerController Object Reference"))
  ;[1 1 1] アイテム獲得時、インベントリにセット
  (bind _asbp_hero (cast `/Game/InGame/Blueprints/Pawns/Characters/BP_Hero` Pawn))
  (`/Game/InGame/Blueprints/Widget/Test/WBP_ItemInventory_test.Add To Inventory` (`/Game/InGame/Blueprints/Pawns/Characters/BP_Hero.WBP_ItemInventory_Test` _asbp_hero) (`self.ItemInfo`)))

(fn `UserConstructionScript`
  (`parent.UserConstructionScript`))