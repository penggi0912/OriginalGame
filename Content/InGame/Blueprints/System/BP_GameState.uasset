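; BP_GameState holds shared progress and mode flags for scroll collection, encounters and target selection.
; HasCompletedLevel reports completion when the first three HasScrolls entries are all true, but ObtainScroll does nothing because its array write is unconnected.
; BeginPlay clears IsEncount, which CreateBattleField only returns without building anything, and TargetSelectMode likewise returns IsTargetSelectMode.
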(event `self.ReceiveBeginPlay`
  (set `self.IsEncount` false))

(fn `CreateBattleField`
  (returns (ReturnValue :type Boolean))
  (return (`self.IsEncount`)))

(fn `HasCompletedLevel`
  (returns (Return :type Boolean))
  (bind _hasscrolls (`self.HasScrolls`))
  (return (and (`|GetArrayItem` _hasscrolls) (`|GetArrayItem` _hasscrolls 1) (`|GetArrayItem` _hasscrolls 2))))

(fn `Obtain Scroll`
  (params (Index :type Integer)))

(fn `TargetSelectMode`
  (returns (Return :type Boolean))
  (return (`self.IsTargetSelectMode`)))

(fn `UserConstructionScript`)