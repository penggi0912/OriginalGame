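; Game mode that initializes the game UI and handles checkpoint respawning.
; On BeginPlay it calls InitGameUI on BP_GameInstance to set up the menu widgets.
; Its FindPlayerStart override returns the Checkpoint stored in BP_GameState when valid, so players respawn there after passing it, and otherwise falls back to the parent's start selection.
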(event `self.ReceiveBeginPlay`
  (bind _asbp_game_instance (cast `/Game/InGame/Blueprints/System/BP_GameInstance` (`GameplayStatics.GetGameInstance`)))
  (`/Game/InGame/Blueprints/System/BP_GameInstance.Init Game UI` _asbp_game_instance) ; メニューウィジェットの初期化
)

(fn `FindPlayerStart`
  (params (Player :type "Controller Object Reference") (IncomingName :type String))
  (returns (ReturnValue :type "Actor Object Reference"))
  (bind _checkpoint (`/Game/InGame/Blueprints/System/BP_GameState.Checkpoint` (cast `/Game/InGame/Blueprints/System/BP_GameState` (`GameplayStatics.GetGameState`) :!pure true)))
  ;[1 1 1] チェックポイント通過後、そこからリスポーン
  (`/Engine/EditorBlueprintResources/StandardMacros.IsValid` _checkpoint
    (:`Is Valid`
      (return _checkpoint))
    (:`Is Not Valid`
      (bind _returnvalue (`parent.FindPlayerStart` Player IncomingName))
      (return _returnvalue))))

(fn `UserConstructionScript`)