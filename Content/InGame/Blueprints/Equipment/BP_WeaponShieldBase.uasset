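; Base shield-weapon Blueprint that displays a hero's equipped shield weapon and animates it when the shield toggles.
; EquipmentName passes the weapon name to a DT_WeaponData lookup, which sets the WeaponShield skeletal mesh and caches its shield animation.
; ShieldActivate plays that montage on the mesh when on, and calls PlayMontage with no montage to stop it when off.
; The hero, damage and item query functions are stubs returning defaults.
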(event `self.ReceiveBeginPlay`)

(event `/Game/InGame/Blueprints/Interfaces/BI_Equipment.Equipment Name`
  (params (Name :type Name))
  ;[1 1 1] シールド用武器のデータ取得
  (bind _output_get (set `self.WeaponName` Name))
  (`self.SetShieldWeaponData_Hero` _output_get))

(event `Shield Activate_2_1`
  (params (`Is Shield On` :type Boolean))
  (bind _weaponshield (`self.WeaponShield`))
  ;[1 1 1] シールドアニメーション
  (if `Is Shield On`
    (`|PlayMontage` _weaponshield (`self.ShieldAnim`)) ; シールドアニメーション開始
    (else
      (`|PlayMontage` _weaponshield) ; 停止
    )))

(fn `Check Invinsible`
  (returns (`IsInvinsible?` :type Boolean))
  (return false))

(fn `CheckHaveDamaged`
  (returns (`HaveDamaged?` :type Boolean))
  (return false))

(fn `Get Attacking Skill Name`
  (returns (SkillName :type Name))
  (return "None"))

(fn `Get Hero Data`
  (returns (`Hero Data` :type "/Game/InGame/Blueprints/Data/Player/ST_HeroData Structure"))
  (return))

(fn `Get Hero HP&MP`
  (returns (MaxHP :type "Float (double-precision)") (CurrentHP :type "Float (double-precision)") (MaxMP :type "Float (double-precision)") (CurrentMP :type "Float (double-precision)"))
  (return 0.0 0.0 0.0 0.0))

(fn `Get Hero Ref`
  (returns (`Hero BP Ref` :type "/Game/InGame/Blueprints/Pawns/Characters/BP_HeroBase Object Reference"))
  (return null))

(fn `Get Hero Weapon Ref`
  (returns (`Hero Weapon Ref` :type "/Game/InGame/Blueprints/Equipment/BP_WeaponBase_Hero Object Reference"))
  (return null))

(fn `Get Use Item Data`
  (returns (`Item Data` :type "/Game/InGame/Blueprints/Data/ST_ItemData Structure"))
  (return))

(fn `SetShieldWeaponData_Hero`
  (params (RowName :type Name))
  (bind _returnvalue (`|GetDataTableRow` "/Game/InGame/Blueprints/Data/Player/DT_WeaponData.DT_WeaponData" RowName) ; 武器名からデータテーブル検索
    (:`then`
      (bind _output_get (set `self.WeaponData` _returnvalue)) ; 武器データセット
      (bind (_name _type _elements _rarity _category _attackvalue _mesh _shieldweapon _shieldanim) (break `/Game/InGame/Blueprints/Data/Player/ST_WeaponData` _output_get))
      (`SkeletalMeshComponent.SetSkeletalMeshAsset` (`self.WeaponShield`) _shieldweapon) ; データテーブルに設定された\nシールド用武器メッシュをセット
      (set `self.ShieldAnim` _shieldanim) ; シールド用武器のアニメーションをセット
    )))

(fn `UserConstructionScript`)