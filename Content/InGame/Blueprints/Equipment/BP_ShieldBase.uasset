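; Base shield actor that registers itself as active when spawned and flashes when hit.
; Its construction script checks the owner for PawnInterface, notifies it and its shield weapon of activation, and caches the original mesh material.
; The hit event swaps in a dynamic instance of the hit material, restores the original after a brief delay, then clears the hit flag by message.
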(event `/Game/InGame/Blueprints/Interfaces/BI_Shield.SetShieldHitted`
  (params (`Is Shield Hitted` :type Boolean))
  (bind _shield (`self.Shield`))
  ;[1 1 1] シールドに攻撃がヒットした時にシールドメッシュのマテリアルを変更
  (if `Is Shield Hitted`
    ;;[1 1 1] ヒット時のマテリアルに変更
    (bind _returnvalue (`PrimitiveComponent.CreateDynamicMaterialInstance` _shield 0 (`self.ShieldHittedMaterial`) "None"))
    (`PrimitiveComponent.SetMaterial` _shield 0 _returnvalue)
    (`KismetSystemLibrary.Delay` 0.2)
    ;;[1 1 1] 元のマテリアルに戻す
    (bind _returnvalue_2 (`PrimitiveComponent.CreateDynamicMaterialInstance` _shield 0 (`self.ShieldMaterial`) "None"))
    (`PrimitiveComponent.SetMaterial` _shield 0 _returnvalue_2)
    (message `/Game/InGame/Blueprints/Interfaces/BI_Shield.SetShieldHitted` self false) ; シールドヒットフラグをオフ
  ))

(fn `Check Shield Activation`
  (returns (`isShieldActivate?` :type Boolean))
  (return (`self.isShieldActivate?`)))

(fn `Check Shield Hitted`
  (returns (`IsShieldHitted?` :type Boolean))
  (return false))

(fn `GetShieldWeaponRef`
  (returns (shieldWeaponRef :type "/Game/InGame/Blueprints/Equipment/BP_WeaponShieldBase Object Reference"))
  (return null))

(fn `UserConstructionScript`
  (bind _returnvalue (`self.GetOwner` self))
  ;[1 1 1] シールドスポーン時の初動
  (if (`KismetSystemLibrary.DoesImplementInterface` _returnvalue (`self.PawnInterface`))
    (bind _output_get (set `self.isShieldActivate?` true)) ; シールド展開フラグオン
    (message `/Game/InGame/Blueprints/Interfaces/BI_Shield.SetShieldActivation` _returnvalue _output_get) ; シールドの所有ポーンへ\nシールドの有効化フラグを通知
    (bind _shieldweaponref (message `/Game/InGame/Blueprints/Interfaces/BI_Shield.GetShieldWeaponRef` _returnvalue)) ; シールド用武器情報を取得
    (bind _output_get_2 (set `self.Weapon Shield Ref` _shieldweaponref))
    (message `/Game/InGame/Blueprints/Interfaces/BI_Shield.SetShieldActivation` _output_get_2 _output_get) ; シールドの所有ポーンへ\nシールドの有効化フラグを通知
    (set `self.ShieldMaterial` (`PrimitiveComponent.GetMaterial` (`self.Shield`) 0)) ; 初期マテリアルをセット
  ))