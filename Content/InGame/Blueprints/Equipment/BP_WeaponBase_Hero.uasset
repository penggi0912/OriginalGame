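; Base Blueprint for hero weapons, which sets up a weapon's data and appearance from its name.
; EquipmentName stores the name and passes it to SetWeaponData_Hero, which looks up DT_WeaponData, caches the row and applies its mesh to the skeletal mesh.
; Hero query functions such as damage, invincibility and HP/MP are stubs returning defaults.
; WeaponChange is empty, and collision-capsule sizing from mesh bounds is left unconnected.
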(event `self.ReceiveBeginPlay`)

(event `self.ReceiveTick`
  (params (DeltaSeconds :type "Float (single-precision)")))

(event `WeaponChange`)

(event `/Game/InGame/Blueprints/Interfaces/BI_Equipment.Equipment Name`
  (params (Name :type Name))
  ;[1 1 1] 武器のクラス名から武器データをセット
  (bind _output_get (set `self.WeaponName` Name))
  (`self.SetWeaponData_Hero` _output_get))

(fn `CheckHasDamaged`
  (returns (`hasDamaged?` :type Boolean))
  (return false))

(fn `CheckInvinsible`
  (returns (`isInvinsible?` :type Boolean))
  (return false))

(fn `GetAttackingSkillName`
  (returns (skillName :type Name))
  (return "None"))

(fn `GetHeroData`
  (returns (heroData :type "/Game/InGame/Blueprints/Data/Player/ST_HeroData Structure"))
  (return))

(fn `GetHeroHP&MP`
  (returns (maxHP :type "Float (double-precision)") (currentHP :type "Float (double-precision)") (maxMP :type "Float (double-precision)") (currentMP :type "Float (double-precision)"))
  (return 0.0 0.0 0.0 0.0))

(fn `GetHeroRef`
  (returns (heroRef :type "/Game/InGame/Blueprints/Pawns/Characters/BP_HeroBase Object Reference"))
  (return null))

(fn `GetHeroWeaponRef`
  (returns (heroWeaponRef :type "/Game/InGame/Blueprints/Equipment/BP_WeaponBase_Hero Object Reference"))
  (return null))

(fn `GetUseItemData`
  (returns (itemData :type "/Game/InGame/Blueprints/Data/ST_ItemData Structure"))
  (return))

(fn `SetWeaponData_Hero`
  (params (`Row Name` :type Name))
  (bind _returnvalue (`|GetDataTableRow` "/Game/InGame/Blueprints/Data/Player/DT_WeaponData.DT_WeaponData" `Row Name`) ; 武器名からデータテーブル検索
    (:`then`
      (bind _output_get (set `self.WeaponData` _returnvalue)) ; 武器データセット
      (`SkeletalMeshComponent.SetSkeletalMeshAsset` (`self.SkeletalMesh`) (`.Mesh_16_4A1F6F16425A84FBC845C98E909602DD` (break `/Game/InGame/Blueprints/Data/Player/ST_WeaponData` _output_get))))))

(fn `UserConstructionScript`)