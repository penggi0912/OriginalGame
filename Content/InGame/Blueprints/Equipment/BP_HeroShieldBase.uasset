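; Base hero shield equipment Blueprint that drives a spear-based shield animation.
; BeginPlay loads the BP_HeroSpear row from DT_PlayerWeaponData into WeaponData.
; ShieldActivate plays Shield_Spear_Montage on the skeletal mesh when on, and calls PlayMontage with no montage when off.
; Item and skill functions are stubs, and a manual spear-spin rotation is left disconnected, noted as a workaround for socket-related animation limits.
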(event `self.ReceiveBeginPlay`
  (bind _returnvalue (`|GetDataTableRow` "/Game/InGame/Blueprints/Data/Player/DT_PlayerWeaponData.DT_PlayerWeaponData" "BP_HeroSpear")
    (:`then`
      (set `self.WeaponData` _returnvalue))))

(event `self.ReceiveTick`
  (params (DeltaSeconds :type "Float (single-precision)")))

(event `/Game/InGame/Blueprints/Interfaces/BI_Hero.Shield Activate`
  (params (`Shield On` :type Boolean))
  (bind _skeletalmesh (`self.SkeletalMesh`))
  (if `Shield On`
    (`|PlayMontage` _skeletalmesh "/Game/InGame/Animation/Characters/Montage/Shield_Spear_Montage.Shield_Spear_Montage")
    (else
      (`|PlayMontage` _skeletalmesh))))

(fn `Use Item Data`
  (params (`Item Data Input` :type "/Game/InGame/Blueprints/Data/ST_ItemData Structure"))
  (returns (`Item Data Output` :type "/Game/InGame/Blueprints/Data/ST_ItemData Structure"))
  (return))

(fn `Use Skill Data`
  (params (SkillNameIn :type Name))
  (returns (SkillNameOut :type Name))
  (return "None"))

(fn `UserConstructionScript`)