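; BP_ShieldBase_Hero is the hero's deployable shield equipment actor, which flashes when hit.
; On construction it marks the shield active, notifies its owner and the hero's shield weapon through ShieldActivateMessage, and caches the original mesh material.
; ShieldDamage swaps in a dynamic instance of the hit material, waits briefly, restores the original and clears the hit flag.
; UseItemData and UseSkillData are empty stubs.
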(event `self.ReceiveBeginPlay`)

(event `/Game/InGame/Blueprints/Interfaces/BI_Hero.Shield Damage`
  (params (`Is Shield Hitted` :type Boolean))
  ;[1 1 1] シールドに攻撃がヒットした時にシールドメッシュのマテリアルを変更
  (if `Is Shield Hitted`
    ;;[1 1 1] ヒット時のマテリアルに変更
    (bind _returnvalue (`PrimitiveComponent.CreateDynamicMaterialInstance` (`self.Shield`) 0 (`self.ShieldHittedMaterial`) "None"))
    (`PrimitiveComponent.SetMaterial` (`self.Shield`) 0 _returnvalue)
    (`KismetSystemLibrary.Delay` 0.2)
    ;;[1 1 1] 元のマテリアルに戻す
    (bind _returnvalue_2 (`PrimitiveComponent.CreateDynamicMaterialInstance` (`self.Shield`) 0 (`self.ShieldMaterial`) "None"))
    (`PrimitiveComponent.SetMaterial` (`self.Shield`) 0 _returnvalue_2)
    (message `/Game/InGame/Blueprints/Interfaces/BI_Hero.Shield Damage` self false) ; シールドヒットフラグをオフ
  ))

(event `self.ReceiveTick`
  (params (DeltaSeconds :type "Float (single-precision)")))

(fn `Use Item Data`
  (params (`Item Data Input` :type "/Game/InGame/Blueprints/Data/ST_ItemData Structure"))
  (returns (`Item Data Output` :type "/Game/InGame/Blueprints/Data/ST_ItemData Structure"))
  (return))

(fn `Use Skill Data`
  (params (SkillNameIn :type Name))
  (returns (SkillNameOut :type Name))
  (return "None"))

(fn `UserConstructionScript`
  (bind _returnvalue (`self.GetOwner` self))
  ;[1 1 1] シールドスポーン時の初動
  (bind _output_get (set `self.IsShieldOn` true)) ; シールド展開フラグオン
  (message `/Game/InGame/Blueprints/Interfaces/BI_Hero.Shield Activate` _returnvalue _output_get) ; シールドの所有ポーンへ通知
  (message `/Game/InGame/Blueprints/Interfaces/BI_Hero.Shield Activate` (`/Game/InGame/Blueprints/Pawns/Characters/BP_HeroBase.WeaponShieldRef` (cast `/Game/InGame/Blueprints/Pawns/Characters/BP_HeroBase` _returnvalue :!pure true)) (`self.IsShieldOn`)) ; シールド用武器BPへ通知
  (set `self.ShieldMaterial` (`PrimitiveComponent.GetMaterial` (`self.Shield`) 0)) ; 初期マテリアルをセット
)