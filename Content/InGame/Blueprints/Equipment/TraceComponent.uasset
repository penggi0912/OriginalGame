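; Actor component that handles weapon hit detection for the hero's attacks against skeleton enemies.
; While the weapon is active, each Tick runs a debug-drawn multi sphere trace between the weapon mesh's start and end sockets.
; It stores each hit actor and location, skips actors in an ignore list and skeletons in invincibility time, then calls the owning hero's damage event.
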(event `self.ReceiveTick`
  (params (DeltaSeconds :type "Float (single-precision)"))
  (bind _weapon_ref (`self.Weapon_Ref`))
  ;[1 1 1] 武器のダメージ判定
  (if (`self.WeaponActive`)
    (`/Engine/EditorBlueprintResources/StandardMacros.IsValid` _weapon_ref
      (:`Is Valid`
        (bind _outhits (`KismetSystemLibrary.SphereTraceMulti` :`Start` (`SceneComponent.GetSocketLocation` (`/Game/InGame/Blueprints/Equipment/BP_HeroSpear.SkeletalMesh` _weapon_ref) "start") :`End` (`SceneComponent.GetSocketLocation` (`/Game/InGame/Blueprints/Equipment/BP_HeroSpear.SkeletalMesh` _weapon_ref) "end") :`Radius` 12.0 :`TraceChannel` "TraceTypeQuery4" :`DrawDebugType` "ForDuration" :`DrawTime` 2.0))
        (for _array_element _outhits
          (bind (_bblockinghit _binitialoverlap _time _distance _location _impactpoint _normal _impactnormal _physmat _hitactor) (`GameplayStatics.BreakHitResult` _array_element))
          (bind _output_get (set `self.Hit Actor` _hitactor))
          (set `self.Location` _location) ; ダメージ表示用に\nヒット箇所の位置取得
          (if (not (`KismetArrayLibrary.Array_Contains` (`self.ActorToIgnore`) _hitactor))
            (bind _asbp_skeleton (cast `/Game/InGame/Blueprints/Pawns/Enemies/BP_Skeleton` _output_get))
            (if (not (`/Game/InGame/Blueprints/Pawns/Enemies/BP_Skeleton.Invinsible Time` _asbp_skeleton))
              (bind _asbp_hero (cast `/Game/InGame/Blueprints/Pawns/Characters/BP_Hero` (`self.GetOwner`)))
              (`/Game/InGame/Blueprints/Pawns/Characters/BP_Hero.Event Apply Damage` _asbp_hero))))))))