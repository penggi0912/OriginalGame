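; AC_SineCurveMovement is an actor component that oscillates its owning actor along a sine wave around its starting position.
; BeginPlay caches the owner's location, and Tick sets the location to that origin plus a per-axis SineCurve offset.
; Amplitude, Period and Phase vectors tune each axis independently, driven by absolute game time rather than accumulated delta, with sweep disabled.
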(event `self.ReceiveBeginPlay`
  (set `self.InitialLocation` (`Actor.K2_GetActorLocation` (`self.GetOwner`))))

(event `self.ReceiveTick`
  (params (DeltaSeconds :type "Float (single-precision)"))
  (bind (_amplitude_x _amplitude_y) (`KismetMathLibrary.BreakVector` (`self.Amplitude`)))
  (bind (_period_x _period_y) (`KismetMathLibrary.BreakVector` (`self.Period`)))
  (bind _phase_x (`KismetMathLibrary.BreakVector` (`self.Phase`)))
  (bind (_phase_x_2 _phase_y) (`KismetMathLibrary.BreakVector` (`self.Phase`)))
  (bind (_amplitude_x_2 _amplitude_y_2 _amplitude_z) (`KismetMathLibrary.BreakVector` (`self.Amplitude`)))
  (bind (_period_x_2 _period_y_2 _period_z) (`KismetMathLibrary.BreakVector` (`self.Period`)))
  (bind (_phase_x_3 _phase_y_2 _phase_z) (`KismetMathLibrary.BreakVector` (`self.Phase`)))
  (bind _amplitude_x_3 (`KismetMathLibrary.BreakVector` (`self.Amplitude`)))
  (bind _period_x_3 (`KismetMathLibrary.BreakVector` (`self.Period`)))
  ;[1 1 1] 正弦波で上下に動かす
  (`Actor.K2_SetActorLocation` (`self.GetOwner`) (+ (`KismetMathLibrary.MakeVector` (`/Game/InGame/Blueprints/Libraries/BP_FuncLibrary.SineCurve` _amplitude_x_3 _period_x_3 (`KismetSystemLibrary.GetGameTimeInSeconds`) _phase_x) (`/Game/InGame/Blueprints/Libraries/BP_FuncLibrary.SineCurve` _amplitude_y _period_y (`KismetSystemLibrary.GetGameTimeInSeconds`) _phase_y) (`/Game/InGame/Blueprints/Libraries/BP_FuncLibrary.SineCurve` _amplitude_z _period_z (`KismetSystemLibrary.GetGameTimeInSeconds`) _phase_z)) (`self.InitialLocation`)) false false))