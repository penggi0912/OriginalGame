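; Actor component that detects melee weapon hits for the hero and passes damage requests back to it.
; While WeaponActive is set, Tick runs a multi-sphere trace between the weapon mesh's start and end sockets.
; For each hit actor not in ActorToIgnore, it stores the location and actor, then calls EventApplyDamage on the hero.
; Hero and weapon references arrive through events; the item and skill functions are empty stubs.
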(event `/Game/InGame/Blueprints/Interfaces/BI_Hero.Hero BP Ref`
  (params (`Hero BP Ref` :type "/Game/InGame/Blueprints/Pawns/Characters/BP_HeroBase Object Reference"))
  (set `self.Hero Ref` `Hero BP Ref`))

(event `/Game/InGame/Blueprints/Interfaces/BI_Hero.Hero Weapon Ref`
  (params (`Hero Weapon Ref` :type "/Game/InGame/Blueprints/Equipment/BP_HeroWeaponBase Object Reference"))
  (set `self.Weapon_Ref` `Hero Weapon Ref`))

(event `self.ReceiveTick`
  (params (DeltaSeconds :type "Float (single-precision)"))
  (bind _weapon_ref (`self.Weapon_Ref`))
  ;[1 1 1] 武器のダメージ判定
  (if (`self.WeaponActive`)
    (`/Engine/EditorBlueprintResources/StandardMacros.IsValid` _weapon_ref
      (:`Is Valid`
        (bind _outhits (`KismetSystemLibrary.SphereTraceMulti` :`Start` (`SceneComponent.GetSocketLocation` (`/Game/InGame/Blueprints/Equipment/BP_HeroWeaponBase.SkeletalMesh` _weapon_ref) "start") :`End` (`SceneComponent.GetSocketLocation` (`/Game/InGame/Blueprints/Equipment/BP_HeroWeaponBase.SkeletalMesh` _weapon_ref) "end") :`Radius` 15.0 :`TraceChannel` "TraceTypeQuery4" :`DrawTime` 2.0)) ; PlayerAttackのトレースをオーバーラップするかどうか
        (for _array_element _outhits
          (bind (_bblockinghit _binitialoverlap _time _distance _location _impactpoint _normal _impactnormal _physmat _hitactor) (`GameplayStatics.BreakHitResult` _array_element))
          (if (not (`KismetArrayLibrary.Array_Contains` (`self.ActorToIgnore`) _hitactor))
            (set `self.Location` _location) ; ダメージ表示とヒット音再生用に\nヒット箇所の位置取得
            (bind _output_get (set `self.Hit Actor` _hitactor))
            (`/Game/InGame/Blueprints/Pawns/Characters/BP_HeroBase.Event Apply Damage` (`self.Hero Ref`) _output_get)))))))

(fn `Use Item Data`
  (params (`Item Data Input` :type "/Game/InGame/Blueprints/Data/ST_ItemData Structure"))
  (returns (`Item Data Output` :type "/Game/InGame/Blueprints/Data/ST_ItemData Structure"))
  (return))

(fn `Use Skill Data`
  (params (SkillNameIn :type Name))
  (returns (SkillNameOut :type Name))
  (return "None"))