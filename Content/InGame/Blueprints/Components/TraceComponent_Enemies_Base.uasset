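; Base trace component for enemies that detects melee attack hits on heroes and their shields.
; While active, Tick picks a sphere trace by skill motion type: weapon sockets, body-part sockets named from the enum, or left/right sockets gated by attack flags.
; Hits outside the ignore list pass through a BI_Hero check, excluding other enemies, into the owning enemy's EventApplyDamage.
; Shield hits notify the shield's owner and target that owner for damage.
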(event `/Game/InGame/Blueprints/Interfaces/BI_Enemy.SetEnemyRef`
  (params (EnemyRef :type "/Game/InGame/Blueprints/Pawns/Enemies/BP_EnemyBase Object Reference"))
  ;[1 1 1] 自身の情報セット
  (set `self.As BP Enemy Base` EnemyRef) ; 自身のポーン情報をセット
  (set `self.ShieldClass` "/Game/InGame/Blueprints/Equipment/BP_ShieldBase_Hero.BP_ShieldBase_Hero_C") ; シールド判定用にプレイヤーの\nシールドクラスをセット
)

(event `/Game/InGame/Blueprints/Interfaces/BI_Enemy.SetEnemyWeaponRef`
  (params (EnemyWeaponRef :type "/Game/InGame/Blueprints/Equipment/BP_WeaponBase_Enemy Object Reference"))
  ;[1 1 1] 武器情報セット
  (set `self.EnemyWeapon_Ref_Trace` EnemyWeaponRef) ; 自身の武器情報をセット
)

(event `/Game/InGame/Blueprints/Interfaces/BI_Enemy.SetEnemySkillMotionType`
  (params (`Skill Motion Type` :type "/Game/InGame/Blueprints/Data/Enum/EN_EnemySkillMotionType Enum" :default "NewEnumerator9"))
  ;[1 1 1] 攻撃部位セット
  (set `self.Skill Motion Type` `Skill Motion Type`) ; エネミーの攻撃部位セット
)

(event `self.ReceiveTick`
  (params (DeltaSeconds :type "Float (single-precision)"))
  ;[1 1 1] ダメージ判定分岐
  (if (`self.EenemyWeaponActive`)
    (switch `/Game/InGame/Blueprints/Data/Enum/EN_EnemySkillMotionType` (`self.Skill Motion Type`) ; スキルモーションタイプ（= 当たり判定発生部位）に応じて\n判定処理を分岐　※PrrojectileはBP側で直接当たり判定
      (:`NewEnumerator9`
        (`self.Begin Trace Weapon`) ; 武器の当たり判定
      )
      (:`NewEnumerator0`
        (`self.Begin Trace FourLegs` :!label _label) ; 四足歩行系エネミーの当たり判定
      )
      (:`NewEnumerator7`
        (`self.Begin Trace Twin` :!label _label_2) ; 左右部位同時攻撃時の当たり判定
      )
      (:`NewEnumerator2`
        (goto _label))
      (:`NewEnumerator1`
        (goto _label))
      (:`NewEnumerator3`
        (goto _label))
      (:`NewEnumerator4`
        (goto _label))
      (:`NewEnumerator12`
        (goto _label_2))
      (:`NewEnumerator10`
        (goto _label))
      (:`NewEnumerator5`
        (goto _label))
      (:`NewEnumerator6`
        (goto _label))
      (:`NewEnumerator8`
        (goto _label)))))

(event `Begin Trace Weapon`
  (bind _enemyweapon_ref_trace (`self.EnemyWeapon_Ref_Trace`))
  (bind _skeletalmesh (`/Game/InGame/Blueprints/Equipment/BP_WeaponBase_Enemy.SkeletalMesh` _enemyweapon_ref_trace))
  ;[1 1 1] 武器所有可能エネミーの攻撃判定。デフォルト
  (`/Engine/EditorBlueprintResources/StandardMacros.IsValid` _enemyweapon_ref_trace ; エネミーの武器が有効かどうかチェック
    (:`Is Valid`
      (bind _outhits (`KismetSystemLibrary.SphereTraceMulti` :`Start` (`SceneComponent.GetSocketLocation` _skeletalmesh "start") :`End` (`SceneComponent.GetSocketLocation` _skeletalmesh "end") :`Radius` 20.0 :`TraceChannel` "TraceTypeQuery3" :`DrawDebugType` "ForDuration")) ; EnemyAttackのトレースをオーバーラップするかどうか
      ;;[1 1 1] ここを関数にするとヒットがループしてしまう。要改修
      (for _array_element _outhits
        (bind (_bblockinghit _binitialoverlap _time _distance _location _impactpoint _normal _impactnormal _physmat _hitactor) (`GameplayStatics.BreakHitResult` _array_element))
        (if (not (`KismetArrayLibrary.Array_Contains` (`self.ActorToIgnore`) _hitactor))
          (set `self.Location` _location) ; ダメージ表示とヒット音再生用に\nヒット箇所の位置取得
          (bind _output_get (set `self.Hit Actor` _hitactor))
          (`self.Check Hit Actor Class E` _output_get) ; Hitアクターがプレイヤーポーンか\nプレイヤーのシールドか判定
        )))))

(event `Begin Trace FourLegs`
  (bind _as_bp_enemy_base (`self.As BP Enemy Base`))
  (bind _skill_motion_type (`self.Skill Motion Type`))
  (bind _mesh (`Character.Mesh` _as_bp_enemy_base))
  ;[1 1 1] 四足歩行系エネミーの当たり判定。スキルに設定したモーションタイプによって、攻撃部位ごとでトレースの発生場所を変える。
  (`/Engine/EditorBlueprintResources/StandardMacros.IsValid` _as_bp_enemy_base
    (:`Is Valid`
      (bind _outhits (`KismetSystemLibrary.SphereTraceMulti` (`SceneComponent.GetSocketLocation` _mesh (`KismetStringLibrary.Conv_StringToName` (`KismetStringLibrary.Concat_StrStr` (`|GetEnumeratorNameAsString` _skill_motion_type) "Start"))) (`SceneComponent.GetSocketLocation` _mesh (`KismetStringLibrary.Conv_StringToName` (`KismetStringLibrary.Concat_StrStr` (`|GetEnumeratorNameAsString` _skill_motion_type) "End"))) 20.0 "TraceTypeQuery3")) ; EnemyAttackのトレースをオーバーラップするかどうか
      (for _array_element _outhits
        (bind (_bblockinghit _binitialoverlap _time _distance _location _impactpoint _normal _impactnormal _physmat _hitactor) (`GameplayStatics.BreakHitResult` _array_element))
        (if (not (`KismetArrayLibrary.Array_Contains` (`self.ActorToIgnore`) _hitactor))
          (set `self.Location` _location) ; ダメージ表示とヒット音再生用に\nヒット箇所の位置取得
          (bind _output_get (set `self.Hit Actor` _hitactor))
          (`self.Check Hit Actor Class E` _output_get) ; Hitアクターがプレイヤーポーンか\nプレイヤーのシールドか判定
        )))))

(event `Begin Trace Twin`
  (bind _as_bp_enemy_base (`self.As BP Enemy Base`))
  (bind _skill_motion_type (`self.Skill Motion Type`))
  (bind _mesh (`Character.Mesh` _as_bp_enemy_base))
  ;[1 1 1] 左右両方の部位で攻撃する時の当たり判定処理。攻撃時にどちらの部位かABP側に通知を送ってフラグをオンにする。
  (`/Engine/EditorBlueprintResources/StandardMacros.IsValid` _as_bp_enemy_base
    (:`Is Valid`
      ;;[1 1 1] 左部位判定有効化
      (if (`self.LeftAttack`)
        (bind _outhits (`KismetSystemLibrary.SphereTraceMulti` (`SceneComponent.GetSocketLocation` _mesh (`KismetStringLibrary.Conv_StringToName` (`KismetStringLibrary.Concat_StrStr` (`|GetEnumeratorNameAsString` _skill_motion_type) "_L" "Start"))) (`SceneComponent.GetSocketLocation` _mesh (`KismetStringLibrary.Conv_StringToName` (`KismetStringLibrary.Concat_StrStr` (`|GetEnumeratorNameAsString` _skill_motion_type) "_L" "End"))) 20.0 "TraceTypeQuery3")) ; EnemyAttackのトレースをオーバーラップするかどうか
        (for _array_element _outhits
          (bind (_bblockinghit _binitialoverlap _time _distance _location _impactpoint _normal _impactnormal _physmat _hitactor) (`GameplayStatics.BreakHitResult` _array_element))
          (if (not (`KismetArrayLibrary.Array_Contains` (`self.ActorToIgnore`) _hitactor))
            (set `self.LeftAttack` false) ; 左部位攻撃解除
            (set `self.Location` _location) ; ダメージ表示とヒット音再生用に\nヒット箇所の位置取得
            (bind _output_get (set `self.Hit Actor` _hitactor))
            (`self.Check Hit Actor Class E` _output_get) ; Hitアクターがプレイヤーポーンか\nプレイヤーのシールドか判定
          ))
        (else
          ;;[1 1 1] 右部位判定有効化
          (if (`self.RightAttack`)
            (bind _outhits_2 (`KismetSystemLibrary.SphereTraceMulti` (`SceneComponent.GetSocketLocation` _mesh (`KismetStringLibrary.Conv_StringToName` (`KismetStringLibrary.Concat_StrStr` (`|GetEnumeratorNameAsString` _skill_motion_type) "_R" "Start"))) (`SceneComponent.GetSocketLocation` _mesh (`KismetStringLibrary.Conv_StringToName` (`KismetStringLibrary.Concat_StrStr` (`|GetEnumeratorNameAsString` _skill_motion_type) "_R" "End"))) 20.0 "TraceTypeQuery3")) ; EnemyAttackのトレースをオーバーラップするかどうか
            (for _array_element_2 _outhits_2
              (bind (_bblockinghit_2 _binitialoverlap_2 _time_2 _distance_2 _location_2 _impactpoint_2 _normal_2 _impactnormal_2 _physmat_2 _hitactor_2) (`GameplayStatics.BreakHitResult` _array_element_2))
              (if (not (`KismetArrayLibrary.Array_Contains` (`self.ActorToIgnore`) _hitactor_2))
                (set `self.RightAttack` false) ; 右部位攻撃解除
                (set `self.Location` _location_2) ; ダメージ表示とヒット音再生用に\nヒット箇所の位置取得
                (bind _output_get_2 (set `self.Hit Actor` _hitactor_2))
                (`self.Check Hit Actor Class E` _output_get_2) ; Hitアクターがプレイヤーポーンか\nプレイヤーのシールドか判定
              ))))))))

(fn `BreakHitResult`
  (params (Location :type "Vector Structure") (`Hit Actor` :type "Actor Object Reference") (Condition :type Boolean))
  (returns (Pawn :type "/Game/InGame/Blueprints/Pawns/Enemies/BP_EnemyBase Object Reference"))
  (set `self.Hit Actor` `Hit Actor`)
  (set `self.Location` Location)
  (if (not Condition)
    (bind _asbp_enemy_base (cast `/Game/InGame/Blueprints/Pawns/Enemies/BP_EnemyBase` (`self.GetOwner`)))
    (return _asbp_enemy_base)))

(fn `Check Hit Actor Class E`
  (params (HitActor :type "Actor Object Reference"))
  ;[1 1 1] エネミーの攻撃のHit対象チェック
  ; 対象がエネミーの場合はダメージ与えない
  ; 対象がシールドの場合はシールドの所有者をHit対象として処理する
  (if (`.bSuccess` (cast `Pawn` HitActor :!pure true))
    ;;[1 1 1] Hit対象がポーンの場合
    (if (`KismetSystemLibrary.DoesImplementInterface` HitActor "/Game/InGame/Blueprints/Interfaces/BI_Hero.BI_Hero_C")
      ;;;[1 1 1] Hit対象がプレイヤーキャラの場合
      (bind _hero_data (message `/Game/InGame/Blueprints/Interfaces/BI_Hero.Get Hero Data` HitActor)) ; Hit対象のステータスを取得
      (bind _isinvinsible_ (message `/Game/InGame/Blueprints/Interfaces/BI_Hero.Check Invinsible` HitActor))
      (bind _newparam (message `/Game/InGame/Blueprints/Interfaces/BI_Shield.Check Shield Activation` HitActor))
      (`/Game/InGame/Blueprints/Pawns/Enemies/BP_Skeleton_Sword.Event Apply Damage` (`self.As BP Enemy Base`) HitActor (`self.Skill Motion Type`) _hero_data _newparam _isinvinsible_) ; エネミーの与ダメージ処理へ
    )
    (else
      ;;[1 1 1] Hit対象がポーン以外の場合
      (if (`KismetMathLibrary.ClassIsChildOf` (`GameplayStatics.GetObjectClass` HitActor) (`self.ShieldClass`))
        ;;;[1 1 1] Hit対象がシールドの場合
        (bind _output_get (set `self.ShieldOwner` (`Actor.GetOwner` (`self.Hit Actor`)))) ; シールドの持ち主をセット
        (if (`KismetSystemLibrary.DoesImplementInterface` _output_get "/Game/InGame/Blueprints/Interfaces/BI_Hero.BI_Hero_C")
          ;;;;[1 1 1] シールドの持ち主がプレイヤーキャラの場合
          (message `/Game/InGame/Blueprints/Interfaces/BI_Shield.SetShieldHitted` _output_get true) ; プレイヤーのシールドに\n攻撃がヒットしたことを通知
          (bind _hero_data_2 (message `/Game/InGame/Blueprints/Interfaces/BI_Hero.Get Hero Data` _output_get)) ; シールドの持ち主のステータスを取得
          (`/Game/InGame/Blueprints/Pawns/Enemies/BP_Skeleton_Sword.Event Apply Damage` (`self.As BP Enemy Base`) _output_get (`self.Skill Motion Type`) _hero_data_2 false false) ; エネミーの与ダメージ処理へ
        )))))

(fn `CheckHaveDamagedEnemy`
  (returns (`HaveDamaged?` :type Boolean))
  (return false))

(fn `GetEnemyHP&MP`
  (returns (MaxHP :type "Float (double-precision)") (CurrentHP :type "Float (double-precision)") (MaxMP :type "Float (double-precision)") (CurrentMP :type "Float (double-precision)"))
  (return 0.0 0.0 0.0 0.0))

(fn `GetEnemyRef`
  (returns (EnemyRef :type "/Game/InGame/Blueprints/Pawns/Enemies/BP_EnemyBase Object Reference"))
  (return null))

(fn `GetEnemySkillMotionType`
  (returns (`Skill Motion Type` :type "/Game/InGame/Blueprints/Data/Enum/EN_EnemySkillMotionType Enum"))
  (return "NewEnumerator9"))

(fn `GetEnemyStatus`
  (returns (EnemyData :type "/Game/InGame/Blueprints/Data/Enemy/ST_EnemyData Structure"))
  (return))

(fn `GetEnemyWeaponRef`
  (returns (EnemyWeaponRef :type "/Game/InGame/Blueprints/Equipment/BP_WeaponBase_Enemy Object Reference"))
  (return null))

(fn `GetProjectileAttackFlg`
  (returns (`IsProjectileAttack?` :type Boolean))
  (return false))