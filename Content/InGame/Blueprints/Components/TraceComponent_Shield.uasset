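; TraceComponent_Shield is an unfinished component meant to detect shield hits for the hero and apply damage.
; Its drafted logic sphere-traces from the shield actor while active, then calls the hero's damage event on hit actors outside an ignore list.
; That trace and the hero and shield setup are disconnected from their events, so none runs.
; The hero and shield query functions are stubs returning empty defaults.
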(event `self.Hero BP Ref`
  (params (`Hero BP Ref` :type "/Game/InGame/Blueprints/Pawns/Characters/BP_HeroBase Object Reference")))

(event `/Game/InGame/Blueprints/Interfaces/BI_Shield.SetShieldActivation`
  (params (shieldActivation :type Boolean)))

(event `self.ReceiveTick`
  (params (DeltaSeconds :type "Float (single-precision)"))
  ;[1 1 1] シールド判定（作成中）　トレースチャンネルの大きさは要再設定
)

(fn `CheckHasDamaged`
  (returns (`hasDamaged?` :type Boolean))
  (return false))

(fn `CheckInvinsible`
  (returns (`isInvinsible?` :type Boolean))
  (return false))

(fn `checkShieldHitted`
  (returns (`IsShieldHitted?` :type Boolean))
  (return false))

(fn `GetAttackingSkillName`
  (returns (skillName :type Name))
  (return "None"))

(fn `GetHeroData`
  (returns (heroData :type "/Game/InGame/Blueprints/Data/Player/ST_HeroData Structure"))
  (return))

(fn `GetHeroHP&MP`
  (returns (maxHP :type "Float (double-precision)") (currentHP :type "Float (double-precision)") (maxMP :type "Float (double-precision)") (currentMP :type "Float (double-precision)"))
  (return 0.0 0.0 0.0 0.0))

(fn `GetHeroRef`
  (returns (heroRef :type "/Game/InGame/Blueprints/Pawns/Characters/BP_HeroBase Object Reference"))
  (return null))

(fn `GetHeroWeaponRef`
  (returns (heroWeaponRef :type "/Game/InGame/Blueprints/Equipment/BP_WeaponBase_Hero Object Reference"))
  (return null))

(fn `getShieldActivation`
  (returns (isShieldActivate :type Boolean))
  (return false))

(fn `GetShieldWeaponRef`
  (returns (shieldWeaponRef :type "/Game/InGame/Blueprints/Equipment/BP_WeaponShieldBase Object Reference"))
  (return null))

(fn `GetUseItemData`
  (returns (itemData :type "/Game/InGame/Blueprints/Data/ST_ItemData Structure"))
  (return))