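; Treasure chest field object that the player opens once with the field action button to receive an item.
; Trigger overlap binds or unbinds ChestOpenEvent on BP_HeroBase and shows or hides a button widget, faked by moving and resizing it out of the chest, with timeline-driven camera facing.
; Opening plays the lid animation, spawns SpawnItem, briefly disables input, then destroys the trigger.
; A separate event tosses ten coins in random directions.
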(event `self.ReceiveBeginPlay`
  ;[1 1 1] ボタンイメージのウィジェットをビューポートに追加
  (bind _returnvalue (`|CreateWidget` "/Game/InGame/Blueprints/Widget/WBP_ActionButton.WBP_ActionButton_C"))
  (set `self.ActionButton` _returnvalue)
  (set `self.ChestClose` true) ; ChestCloseをオン
)

(event `ObtainedItem`
  (params (Pawn :type "Pawn Object Reference") (PlayerController :type "PlayerController Object Reference") (Item :type "/Game/InGame/Blueprints/Pickups/BP_Pickup Class Reference"))
  (bind _returnvalue_location (`KismetMathLibrary.BreakTransform` (`self.GetTransform`)))
  ;[1 1 1] 宝箱に設定したアイテムをスポーン
  (bind _returnvalue (`|SpawnActorFromClass` Item (`self.GetTransform`) "Undefined" "MultiplyWithRoot" null null))
  (`self.K2_SetActorLocation` _returnvalue (+ _returnvalue_location (0.0 0.0 100.0)) false false))

(event `Obtainedlmpl_1`
  (params (Pawn :type "Pawn Object Reference") (PlayerController :type "PlayerController Object Reference"))
  ;[1 1 1] コイン10枚出現処理
  (for _ (range 1 11)
    (`|SpawnActorFromClass` "/Game/InGame/Blueprints/Pickups/BP_Coin.BP_Coin_C" (`self.GetTransform`) "Undefined" "MultiplyWithRoot" null (`KismetMathLibrary.TransformDirection` (`KismetMathLibrary.MakeTransform` (0.0 0.0 0.0) (`KismetMathLibrary.MakeRotator` 0.0 20.0 (`KismetMathLibrary.RandomFloatInRange` 0.0 360.0))) (`self.Toss Velocity`)) true 0.0 null)))

(event `self.Trigger.OnComponentBeginOverlap`
  (params (OverlappedComponent :type "PrimitiveComponent Object Reference") (OtherActor :type "Actor Object Reference") (OtherComp :type "PrimitiveComponent Object Reference") (OtherBodyIndex :type Integer) (bFromSweep :type Boolean) (SweepResult :type "HitResult Structure (by ref)"))
  ;[1 1 1] プレイヤーがオーバーラップするとボタンイメージ表示
  ; ※宝箱に埋め込み→サイズ変更＆上部に位置を移動で臨時再現
  (if (`/Game/InGame/Blueprints/Libraries/BP_FuncLibrary.IsPlayerPawn` OtherActor)
    (bind _asbp_hero_base (cast `/Game/InGame/Blueprints/Pawns/Characters/BP_HeroBase` OtherActor))
    (set `/Game/InGame/Blueprints/Pawns/Characters/BP_HeroBase.ActionCommandActivate` true _asbp_hero_base)
    (if (`self.ChestClose`)
      (`self.ButtonActivate`) ; ボタン表示
      (set `self.IsWidgetActivate` true)
      (`self.PlayButtonRotate`) ; カメラに合わせてボタンを正面に表示
      (bind _asbp_hero_base_2 (cast `/Game/InGame/Blueprints/Pawns/Characters/BP_HeroBase` (`GameplayStatics.GetPlayerPawn` 0)))
      (add `/Game/InGame/Blueprints/Pawns/Characters/BP_HeroBase.FieldAction` _asbp_hero_base_2 (delegate `Chest Open Event`)) ; プレイヤーのアクションボタンにバインド
    )))

(event `Chest Open Event`
  (params (Actor :type "Actor Object Reference"))
  ;[1 1 1] プレイヤーがオーバーラップするとボタンイメージ表示
  ; ※宝箱に埋め込み→サイズ変更＆上部に位置を移動で臨時再現
  (`/Engine/EditorBlueprintResources/StandardMacros.DoOnce` false ; 宝箱が一度だけ開くように制御
    (:`Completed`
      (`self.Chest Open`) ; 宝箱オープン・ボタン非表示
      (set `/Game/InGame/Blueprints/Pawns/Characters/BP_HeroBase.ActionCommandActivate` false (stale `self.Trigger.OnComponentBeginOverlap` _asbp_hero_base_2))
      (`self.ObtainedItem` null null (`self.SpawnItem`))
      (`self.DisableInput` (stale `self.Trigger.OnComponentBeginOverlap` _asbp_hero_base_2) null) ; 宝箱オープン中は入力制御
      (`KismetSystemLibrary.Delay` 1.5)
      (`self.EnableInput` (stale `self.Trigger.OnComponentBeginOverlap` _asbp_hero_base_2) null) ; 入力制御解除
      (`ActorComponent.K2_DestroyComponent` (`self.Trigger`)))))

(event `self.Trigger.OnComponentEndOverlap`
  (params (OverlappedComponent :type "PrimitiveComponent Object Reference") (OtherActor :type "Actor Object Reference") (OtherComp :type "PrimitiveComponent Object Reference") (OtherBodyIndex :type Integer))
  ;[1 1 1] プレイヤーがオーバーラップするとボタンイメージ表示
  ; ※宝箱に埋め込み→サイズ変更＆上部に位置を移動で臨時再現
  (if (`/Game/InGame/Blueprints/Libraries/BP_FuncLibrary.IsPlayerPawn` OtherActor)
    (bind _asbp_hero_base (cast `/Game/InGame/Blueprints/Pawns/Characters/BP_HeroBase` OtherActor))
    (set `/Game/InGame/Blueprints/Pawns/Characters/BP_HeroBase.ActionCommandActivate` false _asbp_hero_base)
    (`self.ButtonInactivate`) ; ボタン非表示
    (set `self.IsWidgetActivate` false)
    (bind _asbp_hero_base_2 (cast `/Game/InGame/Blueprints/Pawns/Characters/BP_HeroBase` (`GameplayStatics.GetPlayerPawn` 0)))
    (remove `/Game/InGame/Blueprints/Pawns/Characters/BP_HeroBase.FieldAction` _asbp_hero_base_2 (delegate `Chest Open Event`)) ; バインド解除\n※一度オーバーラップした宝箱が\n同時に開かないように制御
  ))

(event `PlayButtonRotate`
  (bind _circle_button_rotation (`self.Circle Button Rotation`))
  ;[1 1 1] プレイヤーがオーバーラップするとボタンイメージ表示
  ; ※宝箱に埋め込み→サイズ変更＆上部に位置を移動で臨時再現
  ;;[1 1 1] カメラに合わせてボタンを正面に表示
  (if (and (`self.ChestClose`) (`self.IsWidgetActivate`))
    (`TimelineComponent.Play` _circle_button_rotation)
    (else
      (`TimelineComponent.Stop` _circle_button_rotation))))

(fn `ButtonActivate`
  (bind _button_circle (`self.Button_Circle`))
  (`TimelineComponent.Play` (`self.Circle Button Size`)) ; ボタンサイズ拡大
  (`SceneComponent.K2_SetWorldLocation` _button_circle (+ (`SceneComponent.K2_GetComponentLocation` _button_circle) (0.0 0.0 120.0)) false false) ; ボタンを宝箱の上へ移動
)

(fn `ButtonInactivate`
  (bind _button_circle (`self.Button_Circle`))
  (`TimelineComponent.Reverse` (`self.Circle Button Size`)) ; ボタンサイズ縮小
  (`SceneComponent.K2_SetWorldLocation` _button_circle (- (`SceneComponent.K2_GetComponentLocation` _button_circle) (0.0 0.0 120.0)) false false) ; ボタンを宝箱の中に埋め込む
)

(fn `Can Open`
  (returns (Return :type Boolean))
  (return (`PrimitiveComponent.IsOverlappingActor` (`self.Trigger`) (`GameplayStatics.GetPlayerCharacter` 0))))

(fn `Chest Open`
  (set `self.ChestClose` false) ; ChestCloseをオフ
  (set `self.IsWidgetActivate` false)
  (`self.ButtonInactivate`)
  (`SkeletalMeshComponent.PlayAnimation` (`self.Lid`) "/Game/InGame/Animation/FieldObjects/TreasureChest_Open.TreasureChest_Open" false) ; 蓋が開くアニメーション
)

(fn `Get ItemData`
  (returns (ItemData :type "/Game/InGame/Blueprints/Data/ST_ItemData Structure"))
  (return))

(fn `UserConstructionScript`)