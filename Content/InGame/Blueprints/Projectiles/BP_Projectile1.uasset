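; BP_Projectile1 is a projectile that damages what it hits and explodes.
; The construction script applies Speed as the initial ProjectileMovement speed, with no maximum.
; Each Tick runs a short forward line trace with debug drawing; a hit sends ShieldDamageMessage, spawns explosion effect and sound, then destroys the actor.
; Tick also calls SetLifeSpan every frame, so the lifespan timer keeps restarting.
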(event `self.ReceiveBeginPlay`)

(event `self.ReceiveTick`
  (params (DeltaSeconds :type "Float (single-precision)"))
  (bind _returnvalue (`self.K2_GetActorLocation`))
  (`self.SetLifeSpan` 2.0)
  (bind (_outhit _returnvalue_2) (`KismetSystemLibrary.LineTraceSingle` :`Start` _returnvalue :`End` (+ _returnvalue (* (`self.GetActorForwardVector`) 100.0)) :`TraceChannel` "TraceTypeQuery3" :`DrawDebugType` "ForDuration"))
  (if _returnvalue_2
    (bind _output_get (set `self.Hit Actor` (`.HitActor` (`GameplayStatics.BreakHitResult` _outhit))))
    (message `/Game/InGame/Blueprints/Interfaces/BI_Hero.Shield Damage` _output_get false)
    (`GameplayStatics.SpawnEmitterAtLocation` "/Game/StarterContent/Particles/P_Explosion.P_Explosion" (`self.K2_GetActorLocation`))
    (`GameplayStatics.PlaySound2D` "/Game/StarterContent/Audio/Explosion01.Explosion01" 1.0 1.0 0.0 null null)
    (`self.K2_DestroyActor`)))

(fn `UserConstructionScript`
  (bind _projectilemovement (`self.ProjectileMovement`))
  (set `ProjectileMovementComponent.InitialSpeed` (`self.Speed`) _projectilemovement)
  (set `ProjectileMovementComponent.MaxSpeed` 0.0 _projectilemovement))