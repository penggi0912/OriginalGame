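; Base projectile actor for hero and enemy ranged attacks, held at zero speed and gravity until CheckReadytoFire launches it with a short lifespan.
; Box overlap runs a forward multi box trace, passing hits outside ActorToIgnore to CheckHitActorByProjectile.
; That function uses interfaces to filter friendly fire, resolves shield hits to their owners, and delegates damage to the shooter's ProjectileApplyDamage.
; Non-pawn, non-shield hits destroy the projectile with effect and sound.
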(event `self.ReceiveBeginPlay`
  (bind _output_get (set `self.projectileOwner` (`self.GetOwner`)))
  (`PrimitiveComponent.IgnoreActorWhenMoving` (`self.BoxCollision`) _output_get true) ; 使用者が発射後に動いてもコリジョンは無視
)

(event `/Game/InGame/Blueprints/Interfaces/BI_Projectile.checkReadyToFire`
  (params (isReadyToFire :type Boolean))
  (bind _projectilemovement (`self.ProjectileMovement`))
  (bind _output_get (set `self.isReadyToFire` isReadyToFire))
  (if _output_get
    (set `ProjectileMovementComponent.InitialSpeed` (`self.Speed`) _projectilemovement)
    (set `ProjectileMovementComponent.MaxSpeed` (`self.Speed`) _projectilemovement)
    (set `ProjectileMovementComponent.ProjectileGravityScale` (`self.Gravity`) _projectilemovement)
    (`self.SetLifeSpan` 2.0)))

(event `self.BoxCollision.OnComponentBeginOverlap`
  (params (OverlappedComponent :type "PrimitiveComponent Object Reference") (OtherActor :type "Actor Object Reference") (OtherComp :type "PrimitiveComponent Object Reference") (OtherBodyIndex :type Integer) (bFromSweep :type Boolean) (SweepResult :type "HitResult Structure (by ref)"))
  (bind _returnvalue (`SceneComponent.K2_GetComponentLocation` (`self.BoxCollision`)))
  ;[1 1 1] 飛び道具の攻撃判定
  (bind _outhits (`KismetSystemLibrary.BoxTraceMulti` :`Start` _returnvalue :`End` (+ _returnvalue (* (`SceneComponent.GetForwardVector` (`self.BoxCollision`)) 100.0)) :`HalfSize` (`BoxComponent.GetScaledBoxExtent` (`self.BoxCollision`)) :`TraceChannel` "TraceTypeQuery8" :`DrawDebugType` "ForDuration")) ; ProjectileAttackのトレースチャンネルを\nオーバーラップするかどうか
  ;;[1 1 1] ここを関数にするとヒットがループしてしまう。要改修
  (for _array_element _outhits
    (bind (_bblockinghit _binitialoverlap _time _distance _location _impactpoint _normal _impactnormal _physmat _hitactor) (`GameplayStatics.BreakHitResult` _array_element))
    (if (not (`KismetArrayLibrary.Array_Contains` (`self.actorToIgnore`) _hitactor))
      (set `self.location` _location) ; ダメージ表示とヒット音再生用に\nヒット箇所の位置取得
      (bind _output_get (set `self.hitActor` _hitactor))
      (`self.CheckHitActorByProjectile` _output_get (`self.projectileOwner`)) ; Hitアクターがプレイヤーかエネミーかの判定処理
    )))

(event `Destroy Projectile`
  ;[1 1 1] 飛び道具の攻撃判定
  ;;[1 1 1] 弾丸破壊処理
  (set `self.isReadyToFire` false)
  (`GameplayStatics.SpawnEmitterAtLocation` (`self.hitEffect`) (`self.K2_GetActorLocation`)) ; ヒット時のエフェクト再生
  (`GameplayStatics.PlaySound2D` (`self.hitSound`) 1.0 1.0 0.0 null null)
  (`self.K2_DestroyActor`))

(event `self.ReceiveTick`
  (params (DeltaSeconds :type "Float (single-precision)")))

(fn `CheckHitActorByProjectile`
  (params (HitActor :type "Actor Object Reference") (Owner :type "Actor Object Reference"))
  (if (`KismetSystemLibrary.DoesImplementInterface` Owner "/Game/InGame/Blueprints/Interfaces/BI_Hero.BI_Hero_C")
    ;[1 1 1] プレイヤーキャラの弾丸の場合
    (bind _heroref (message `/Game/InGame/Blueprints/Interfaces/BI_Hero.GetHeroRef` Owner)) ; 弾丸の所有者であるプレイヤーキャラの\nBP情報を取得
    (set `self.heroRef` _heroref)
    (if (`.bSuccess` (cast `Pawn` HitActor :!pure true))
      ;;[1 1 1] Hit対象がポーンの場合
      (if (`KismetSystemLibrary.DoesImplementInterface` HitActor "/Game/InGame/Blueprints/Interfaces/BI_Enemy.BI_Enemy_C")
        ;;;[1 1 1] Hit対象がエネミーの場合
        (bind _isenemyinvinsible_ (message `/Game/InGame/Blueprints/Interfaces/BI_Enemy.CheckInvinsibleEnemy` HitActor)) ; エネミーの\n無敵フラグを取得
        (bind _isshieldactivate_ (message `/Game/InGame/Blueprints/Interfaces/BI_Shield.Check Shield Activation` HitActor)) ; エネミーの\nシールド展開フラグを取得
        (bind _enemydata (message `/Game/InGame/Blueprints/Interfaces/BI_Enemy.GetEnemyData` HitActor)) ; エネミーのステータスを取得
        (`/Game/InGame/Blueprints/Pawns/Characters/BP_HeroBase.Projectile Apply Damage` (`self.heroRef`) HitActor _enemydata _isshieldactivate_ _isenemyinvinsible_) ; プレイヤーの与ダメージ処理へ
      )
      (else
        ;;[1 1 1] Hit対象がポーン以外の場合
        (if (`KismetMathLibrary.ClassIsChildOf` (`GameplayStatics.GetObjectClass` HitActor) (`self.shieldClass`))
          ;;;[1 1 1] Hit対象がシールドの場合
          (bind _output_get (set `self.shieldOwner` (`self.GetOwner` (`self.hitActor`)))) ; シールドの持ち主をセット
          (if (`KismetSystemLibrary.DoesImplementInterface` _output_get "/Game/InGame/Blueprints/Interfaces/BI_Enemy.BI_Enemy_C")
            ;;;;[1 1 1] シールドの持ち主がエネミーの場合
            (message `/Game/InGame/Blueprints/Interfaces/BI_Shield.SetShieldHitted` (`self.hitActor`) true) ; エネミーのシールドに\n攻撃がヒットしたことを通知
            (bind _isenemyinvinsible__2 (message `/Game/InGame/Blueprints/Interfaces/BI_Enemy.CheckInvinsibleEnemy` _output_get)) ; シールドの持ち主の\n無敵フラグを取得
            (bind _isshieldactivate__2 (message `/Game/InGame/Blueprints/Interfaces/BI_Shield.Check Shield Activation` _output_get)) ; シールドの持ち主の\nシールド展開フラグを取得
            (bind _enemydata_2 (message `/Game/InGame/Blueprints/Interfaces/BI_Enemy.GetEnemyData` _output_get)) ; シールドの持ち主のステータスを取得
            (`/Game/InGame/Blueprints/Pawns/Characters/BP_HeroBase.Projectile Apply Damage` (`self.heroRef`) _output_get _enemydata_2 _isshieldactivate__2 _isenemyinvinsible__2) ; プレイヤーの与ダメージ処理へ
          )
          (else
            (`self.Destroy Projectile`)))))
    (else
      ;[1 1 1] エネミーの弾丸の場合
      (if (`KismetSystemLibrary.DoesImplementInterface` Owner "/Game/InGame/Blueprints/Interfaces/BI_Enemy.BI_Enemy_C")
        (bind _enemyref (message `/Game/InGame/Blueprints/Interfaces/BI_Enemy.GetEnemyRef` Owner)) ; 弾丸の所有者であるエネミーの\nBP情報を取得
        (set `self.enemyRef` _enemyref)
        (if (`.bSuccess` (cast `Pawn` HitActor :!pure true))
          ;;[1 1 1] Hit対象がポーンの場合
          (if (`KismetSystemLibrary.DoesImplementInterface` HitActor "/Game/InGame/Blueprints/Interfaces/BI_Hero.BI_Hero_C")
            ;;;[1 1 1] Hit対象がプレイヤーキャラの場合
            (bind _isinvinsible_ (message `/Game/InGame/Blueprints/Interfaces/BI_Hero.CheckInvinsible` HitActor)) ; プレイヤーキャラの\n無敵フラグ取得
            (bind _isshieldactivate__3 (message `/Game/InGame/Blueprints/Interfaces/BI_Shield.Check Shield Activation` HitActor)) ; プレイヤーキャラの\nシールド展開フラグ取得
            (bind _herodata (message `/Game/InGame/Blueprints/Interfaces/BI_Hero.GetHeroData` HitActor)) ; プレイヤーキャラの\nステータスを取得
            (`/Game/InGame/Blueprints/Pawns/Enemies/BP_EnemyBase.Projectile Apply Damage` (`self.enemyRef`) HitActor "NewEnumerator17" _herodata _isshieldactivate__3 _isinvinsible_) ; エネミーの与ダメージ処理へ
          )
          (else
            ;;[1 1 1] Hit対象がポーン以外の場合
            (if (`KismetMathLibrary.ClassIsChildOf` (`GameplayStatics.GetObjectClass` HitActor) (`self.shieldClass`))
              ;;;[1 1 1] Hit対象がシールドの場合
              (bind _output_get_2 (set `self.shieldOwner` (`self.GetOwner` (`self.hitActor`)))) ; シールドの持ち主をセット
              (if (`KismetSystemLibrary.DoesImplementInterface` _output_get_2 "/Game/InGame/Blueprints/Interfaces/BI_Hero.BI_Hero_C")
                ;;;;[1 1 1] シールドの持ち主がプレイヤーキャラの場合
                (message `/Game/InGame/Blueprints/Interfaces/BI_Shield.SetShieldHitted` (`self.hitActor`) true) ; プレイヤーのシールドに\n攻撃がヒットしたことを通知
                (bind _isinvinsible__2 (message `/Game/InGame/Blueprints/Interfaces/BI_Hero.CheckInvinsible` _output_get_2)) ; シールドの持ち主の\n無敵フラグを取得
                (bind _isshieldactivate__4 (message `/Game/InGame/Blueprints/Interfaces/BI_Shield.Check Shield Activation` _output_get_2)) ; シールドの持ち主の\nシールド展開フラグを取得
                (bind _herodata_2 (message `/Game/InGame/Blueprints/Interfaces/BI_Hero.GetHeroData` _output_get_2)) ; シールドの持ち主のステータスを取得
                (`/Game/InGame/Blueprints/Pawns/Enemies/BP_EnemyBase.Projectile Apply Damage` (`self.enemyRef`) _output_get_2 "NewEnumerator17" _herodata_2 _isshieldactivate__4 _isinvinsible__2) ; エネミーの与ダメージ処理へ
              )
              (else
                (`self.Destroy Projectile`)))))))))

(fn `UserConstructionScript`
  (bind _projectilemovement (`self.ProjectileMovement`))
  (set `ProjectileMovementComponent.InitialSpeed` 0.0 _projectilemovement)
  (set `ProjectileMovementComponent.MaxSpeed` 0.0 _projectilemovement)
  (set `ProjectileMovementComponent.ProjectileGravityScale` 0.0 _projectilemovement)
  (set `self.shieldClass` "/Game/InGame/Blueprints/Equipment/BP_ShieldBase.BP_ShieldBase_C")
  (`KismetArrayLibrary.Array_Clear` (`self.actorToIgnore`)))