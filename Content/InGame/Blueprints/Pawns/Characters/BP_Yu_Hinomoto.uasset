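; Playable hero character Blueprint for Yu Hinomoto, with spear combo attacks, skills and a work-in-progress teleport dodge.
; Combo attacks and Skill1 read DT_HeroSkillData rows to play montages and display skill names; Skill2 plays a test montage.
; The dodge timeline sweeps Yu forward while driving Opacity on BeginPlay-created dynamic materials and Niagara particle size.
; SetHeroWeaponRef disables weapon collision and destroys the weapon, stowing it for shield use.
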(event `self.ReceiveBeginPlay`
  ;[1 1 1] メッシュのマテリアルでダイナミックマテリアルインスタンス作成、変数化(瞬間移動などのエフェクト用)
  (`parent.ReceiveBeginPlay`)
  (bind _returnvalue (`KismetMaterialLibrary.CreateDynamicMaterialInstance` "/Game/InGame/Meshes/Characters/Yu_Battle/M_N00_000_00_FaceMouth_00_FACE__Instance_.M_N00_000_00_FaceMouth_00_FACE__Instance_"))
  (set `self.FaceMouth` _returnvalue)
  (bind _returnvalue_2 (`KismetMaterialLibrary.CreateDynamicMaterialInstance` "/Game/InGame/Meshes/Characters/Yu_Battle/M_N00_000_00_EyeIris_00_EYE__Instance_.M_N00_000_00_EyeIris_00_EYE__Instance_"))
  (set `self.EyeIris` _returnvalue_2)
  (bind _returnvalue_3 (`KismetMaterialLibrary.CreateDynamicMaterialInstance` "/Game/InGame/Meshes/Characters/Yu_Battle/M_N00_000_00_EyeHighlight_00_EYE__Instance_.M_N00_000_00_EyeHighlight_00_EYE__Instance_"))
  (set `self.EyeHighlight` _returnvalue_3)
  (bind _returnvalue_4 (`KismetMaterialLibrary.CreateDynamicMaterialInstance` "/Game/InGame/Meshes/Characters/Yu_Battle/M_N00_000_00_Face_00_SKIN__Instance_.M_N00_000_00_Face_00_SKIN__Instance_"))
  (set `self.Face` _returnvalue_4)
  (bind _returnvalue_5 (`KismetMaterialLibrary.CreateDynamicMaterialInstance` "/Game/InGame/Meshes/Characters/Yu_Battle/M_N00_000_00_EyeWhite_00_EYE__Instance_.M_N00_000_00_EyeWhite_00_EYE__Instance_"))
  (set `self.EyeWhite` _returnvalue_5)
  (bind _returnvalue_6 (`KismetMaterialLibrary.CreateDynamicMaterialInstance` "/Game/InGame/Meshes/Characters/Yu_Battle/M_N00_000_00_FaceBrow_00_FACE__Instance_.M_N00_000_00_FaceBrow_00_FACE__Instance_"))
  (set `self.FaceBrow` _returnvalue_6)
  (bind _returnvalue_7 (`KismetMaterialLibrary.CreateDynamicMaterialInstance` "/Game/InGame/Meshes/Characters/Yu_Battle/M_N00_000_00_FaceEyeline_00_FACE__Instance_.M_N00_000_00_FaceEyeline_00_FACE__Instance_"))
  (set `self.FaceEyeline` _returnvalue_7)
  (bind _returnvalue_8 (`KismetMaterialLibrary.CreateDynamicMaterialInstance` "/Game/InGame/Meshes/Characters/Yu_Battle/M_N00_000_00_Body_00_SKIN__Instance_.M_N00_000_00_Body_00_SKIN__Instance_"))
  (set `self.Body` _returnvalue_8)
  (bind _returnvalue_9 (`KismetMaterialLibrary.CreateDynamicMaterialInstance` "/Game/InGame/Meshes/Characters/Yu_Battle/M_N00_007_02_Tops_01_CLOTH__Instance_.M_N00_007_02_Tops_01_CLOTH__Instance_"))
  (set `self.Tops` _returnvalue_9)
  (bind _returnvalue_10 (`KismetMaterialLibrary.CreateDynamicMaterialInstance` "/Game/InGame/Meshes/Characters/Yu_Battle/M_N00_001_03_Bottoms_01_CLOTH__Instance_.M_N00_001_03_Bottoms_01_CLOTH__Instance_"))
  (set `self.Bottoms` _returnvalue_10)
  (bind _returnvalue_11 (`KismetMaterialLibrary.CreateDynamicMaterialInstance` "/Game/InGame/Meshes/Characters/Yu_Battle/M_N00_001_01_Shoes_01_CLOTH__Instance_.M_N00_001_01_Shoes_01_CLOTH__Instance_"))
  (set `self.Shoes` _returnvalue_11)
  (bind _returnvalue_12 (`KismetMaterialLibrary.CreateDynamicMaterialInstance` "/Game/InGame/Meshes/Characters/Yu_Battle/M_N00_001_02_Accessory_Tie_01_CLOTH__Instance_.M_N00_001_02_Accessory_Tie_01_CLOTH__Instance_"))
  (set `self.Accessory_Tie` _returnvalue_12)
  (bind _returnvalue_13 (`KismetMaterialLibrary.CreateDynamicMaterialInstance` "/Game/InGame/Meshes/Characters/Yu_Battle/M_N00_000_00_HairBack_00_HAIR__Instance_.M_N00_000_00_HairBack_00_HAIR__Instance_"))
  (set `self.HairBack` _returnvalue_13)
  (bind _returnvalue_14 (`KismetMaterialLibrary.CreateDynamicMaterialInstance` "/Game/InGame/Meshes/Characters/Yu_Battle/M_N00_000_Hair_00_HAIR__Instance_.M_N00_000_Hair_00_HAIR__Instance_"))
  (set `self.Hair` _returnvalue_14)
  (bind _output_get (set `self.MaterialArray` (`|MakeArray` (`self.FaceMouth`) (`self.EyeIris`) (`self.EyeHighlight`) (`self.Face`) (`self.EyeWhite`) (`self.FaceBrow`) (`self.FaceEyeline`) (`self.Body`) (`self.Tops`) (`self.Bottoms`) (`self.Shoes`) (`self.Accessory_Tie`) (`self.HairBack`) (`self.Hair`))))
  (for (_array_element _array_index) _output_get
    (`PrimitiveComponent.SetMaterial` (`self.Mesh`) _array_index _array_element) ; 各メッシュのマテリアルを消す
  )
  (`SceneComponent.SetVisibility` (`self.NS_SkeletalParticle`) false false) ; パーティクルエフェクトを非表示
)

(event `/Game/InGame/Blueprints/Interfaces/BI_Hero.SetHeroWeaponRef`
  (params (weaponRef :type "/Game/InGame/Blueprints/Equipment/BP_WeaponBase_Hero Object Reference"))
  ;[1 1 1] シールド展開(武器をシールドとして使用するため一時格納)
  (`PrimitiveComponent.SetCollisionEnabled` (`/Game/InGame/Blueprints/Equipment/BP_WeaponBase_Hero.WeaponCollision` weaponRef) "NoCollision") ; 念のため武器のコリジョン無効化
  (`self.K2_DestroyActor` weaponRef) ; 武器破壊(=格納)
)

(event `self.Primary Attack Combo1`
  ;[1 1 1] 通常攻撃コンボ
  (bind _returnvalue (`|GetDataTableRow` "/Game/InGame/Blueprints/Data/Player/DT_HeroSkillData.DT_HeroSkillData" "Primary_Attack_A_Spear_Montage_Yu")
    (:`then`
      (set `self.AttackingSkillData` _returnvalue)
      (bind (_skillname _animmontage _atk_multiplier _atk_fixvalue _consumptionmp _type) (break `/Game/InGame/Blueprints/Data/Player/ST_HeroSkillData` _returnvalue))
      (`self.PlayAnimMontage` _animmontage)
      (`self.ViewCurrentSkillName` _skillname _type) ; スキル名表示(通常攻撃は非表示)
    )))

(event `self.Primary Attack Combo2`
  ;[1 1 1] 通常攻撃コンボ
  (bind _returnvalue (`|GetDataTableRow` "/Game/InGame/Blueprints/Data/Player/DT_HeroSkillData.DT_HeroSkillData" "Primary_Attack_B_Spear_Montage_Yu")
    (:`then`
      (set `self.AttackingSkillData` _returnvalue)
      (bind (_skillname _animmontage _atk_multiplier _atk_fixvalue _consumptionmp _type) (break `/Game/InGame/Blueprints/Data/Player/ST_HeroSkillData` _returnvalue))
      (`self.PlayAnimMontage` _animmontage)
      (`self.ViewCurrentSkillName` _skillname _type))))

(event `self.Primary Attack Combo3`
  ;[1 1 1] 通常攻撃コンボ
  (bind _returnvalue (`|GetDataTableRow` "/Game/InGame/Blueprints/Data/Player/DT_HeroSkillData.DT_HeroSkillData" "Primary_Attack_C_Spear_Montage_Yu")
    (:`then`
      (set `self.AttackingSkillData` _returnvalue)
      (bind (_skillname _animmontage _atk_multiplier _atk_fixvalue _consumptionmp _type) (break `/Game/InGame/Blueprints/Data/Player/ST_HeroSkillData` _returnvalue))
      (`self.PlayAnimMontage` _animmontage)
      (`self.ViewCurrentSkillName` _skillname _type))))

(event `self.Skill1`
  ;[1 1 1] スキル1(L1+□/1ボタン)使用
  (bind _returnvalue (`|GetDataTableRow` "/Game/InGame/Blueprints/Data/Player/DT_HeroSkillData.DT_HeroSkillData" "Ability_E1_Montage_Yu")
    (:`then`
      (set `self.AttackingSkillData` _returnvalue)
      (bind (_skillname _animmontage _atk_multiplier _atk_fixvalue _consumptionmp _type) (break `/Game/InGame/Blueprints/Data/Player/ST_HeroSkillData` _returnvalue))
      (`self.PlayAnimMontage` _animmontage)
      (`self.ViewCurrentSkillName` _skillname _type) ; スキル名表示
    )))

(event `self.Skill2`
  ;[1 1 1] スキル2(L1+△/2ボタン)使用
  (`self.PlayAnimMontage` "/Game/InGame/Animation/Characters/Montage/Primary_Attack_Spear_test_Montage_Yu.Primary_Attack_Spear_test_Montage_Yu") ; 仮データ
)

(event `self.Avoid Action`
  ;[1 1 1] 瞬間移動回避アクション（作成中）
  (set `self.InicialLocation` (`self.K2_GetActorLocation`))
  (`SceneComponent.SetVisibility` (`self.NS_SkeletalParticle`) true false)
  (`|PlayMontage` (`self.Mesh`) "/Game/InGame/Animation/Characters/Montage/Running_Slide_Yu_Montage.Running_Slide_Yu_Montage"
    (:`then`
      (bind (_direction _distance_rate _opacity) (`Timeline|タイムライン` :!via `PlayFromStart`)
        (:`Update`
          (`self.K2_SetActorLocation` (+ (* (`self.GetActorForwardVector`) (* _distance_rate 1000.0)) (`self.InicialLocation`)) true)
          (for _array_element (`self.MaterialArray`)
            (`MaterialInstanceDynamic.SetScalarParameterValue` _array_element "Opacity" _opacity)
            (`FXSystemComponent.SetFloatParameter` (`self.NS_SkeletalParticle`) "Particle_Size" (* _opacity 10.0))
            (`self.End Avoid`) ; 回避終了後の挙動
          ))
        (:`Finished`
          (`SceneComponent.SetVisibility` (`self.NS_SkeletalParticle`) false false))))))

(fn `UserConstructionScript`
  (`parent.UserConstructionScript`))