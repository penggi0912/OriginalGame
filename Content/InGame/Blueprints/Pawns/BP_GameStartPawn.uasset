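; BP_GameStartPawn is the pawn that brings up the game's start screen.
; On BeginPlay it adds the default Enhanced Input mapping context to the BP_PlayerController's local player subsystem.
; It then creates WBP_GameStart, adds it to the viewport with the main menu bar color hidden, and sets Game and UI input focused on the Start button.
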(event `self.ReceiveBeginPlay`
  (bind _returnvalue (`GameplayStatics.GetPlayerController` 0))
  (bind _asbp_player_controller (cast `/Game/InGame/Blueprints/System/BP_PlayerController` _returnvalue))
  (bind _returnvalue_2 (pcsubsystem `EnhancedInputLocalPlayerSubsystem` _asbp_player_controller))
  (`/Engine/EditorBlueprintResources/StandardMacros.IsValid` _returnvalue_2
    (:`Is Valid`
      (`EnhancedInputSubsystemInterface.AddMappingContext` _returnvalue_2 "/Game/InGame/AI/Input/IMC_Default.IMC_Default" 0 (struct))
      (bind _returnvalue_3 (`|CreateWidget` "/Game/InGame/Blueprints/Widget/WBP_GameStart.WBP_GameStart_C"))
      (bind _output_get (set `self.WBP_GameStart` _returnvalue_3))
      (`UserWidget.AddToViewport` _output_get 0)
      (`Widget.SetRenderOpacity` (`/Game/InGame/Blueprints/Widget/WBP_GameStart.MainMenu_BarColor` _returnvalue_3) 0.0)
      (`WidgetBlueprintLibrary.SetInputMode_GameAndUIEx` _returnvalue (`/Game/InGame/Blueprints/Widget/WBP_GameStart.StartButton` _returnvalue_3)))))

(fn `UserConstructionScript`)