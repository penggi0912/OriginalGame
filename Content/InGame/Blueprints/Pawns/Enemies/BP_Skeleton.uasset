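; Sword-wielding skeleton enemy that loads stats from DT_EnemyData, runs BT_Enemy and attaches a spawned sword.
; Attack plays a random montage whose asset name keys its DT_EnemySkillData row, displaying non-normal skill names on screen.
; Sword trace hits on BP_Hero apply attack-minus-defence damage with floating numbers, ignoring hit actors until cleared.
; Incoming damage drives the HP bar, hit reaction and one-time death; helpers handle walk/sprint speeds and targetability.
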(event `self.ReceiveBeginPlay`
  ;[1 1 1] ステータス取得
  (bind _returnvalue (`|GetDataTableRow` "/Game/InGame/Blueprints/Data/DT_EnemyData.DT_EnemyData" "Skeleton_Sword")
    (:`then`
      (bind _output_get (set `self.EnemyData` _returnvalue))
      ;;[1 1 1] HP/MPバーウィジェット用にセット
      (set `self.MaxHP` (`.MaxMP_83_6F3610D84A793D6FA33D75B367498554` (break `/Game/InGame/Blueprints/Data/ST_EnemyData` _output_get)))
      (set `self.HP` (`.HP_37_672C45B64AB6932A57B970BF15C8D9E9` (break `/Game/InGame/Blueprints/Data/ST_EnemyData` _output_get)))
      ;[1 1 1] AI System
      (`AIController.RunBehaviorTree` (`AIBlueprintHelperLibrary.GetAIController` self) "/Game/InGame/AI/BehaviorTree/BT_Enemy.BT_Enemy")
      ;[1 1 1] 武器装着
      (bind _returnvalue_2 (`|SpawnActorFromClass` "/Game/InGame/Blueprints/Equipment/BP_EnemySword.BP_EnemySword_C" (`SceneComponent.GetSocketTransform` (`self.Mesh`) "weapon_r" "RTS_World") "Undefined" "MultiplyWithRoot" null null))
      (bind _output_get_2 (set `self.EnemyWeaponref` _returnvalue_2))
      (`self.K2_AttachToComponent` _output_get_2 (`self.Mesh`) "weapon_r" "SnapToTarget" "SnapToTarget" "SnapToTarget" true)
      (set `/Game/InGame/Blueprints/Equipment/TraceComponent_Enemeies.EnemyWeapon_Ref` (`self.EnemyWeaponref`) (`self.TraceComponent_Enemeies`))
      ;[1 1 1] HPバーウィジェット呼び出し
      (bind _aswbp_enemy_hp_bar (cast `/Game/InGame/Blueprints/Widget/In_Battle/WBP_EnemyHP_Bar` (`WidgetComponent.GetWidget` (`self.HP_Bar`))))
      (bind _output_get_3 (set `self.As WBP Enemy HP Bar` _aswbp_enemy_hp_bar))
      (set `/Game/InGame/Blueprints/Widget/In_Battle/WBP_EnemyHP_Bar.Enemy_ref` self _output_get_3)
      (bind _returnvalue_3 (`|CreateWidget` "/Game/InGame/Blueprints/Widget/In_Battle/WBP_EnemySkillName.WBP_EnemySkillName_C"))
      (set `self.WBP_SkillName` _returnvalue_3))))

(event `self.ReceiveAnyDamage`
  (params (Damage :type "Float (single-precision)") (DamageType :type "DamageType Object Reference") (InstigatedBy :type "Controller Object Reference") (DamageCauser :type "Actor Object Reference"))
  (bind (_enemydata_name _enemydata_enemylevel _enemydata_earnexp _enemydata_maxhp _enemydata_hp) (break `/Game/InGame/Blueprints/Data/ST_EnemyData` (`self.EnemyData`)))
  (bind _hp_bar (`self.HP_Bar`))
  ;[1 1 1] 非ダメージ/死亡時の処理
  (set `self.IsDamaged` true)
  (bind _output_get (set `self.EnemyData` (make `/Game/InGame/Blueprints/Data/ST_EnemyData` "None" 1 0.0 0.0 (- _enemydata_hp Damage))))
  (`KismetSystemLibrary.PrintString` "Hello" true true (struct :`R` 1.0 :`G` 0.126427 :`B` 0.246205 :`A` 1.0)) ; デバッグ用残りHP表示
  (if (<= (`.HP_37_672C45B64AB6932A57B970BF15C8D9E9` (break `/Game/InGame/Blueprints/Data/ST_EnemyData` _output_get)) 0.0)
    (`SceneComponent.SetVisibility` _hp_bar false false) ; HPバー非表示
    (`/Engine/EditorBlueprintResources/StandardMacros.DoOnce` false ; 死亡処理は一度だけ実行
      (:`Completed`
        (`BrainComponent.StopLogic` (`AIController.BrainComponent` (`AIBlueprintHelperLibrary.GetAIController` self)) "") ; 死亡後に動かないようロジック停止
        (`self.PlayAnimMontage` "/Game/InGame/Animation/Enemies/Montage/Skele_Death_Montage.Skele_Death_Montage")
        (`CharacterMovementComponent.DisableMovement` (`self.CharacterMovement`)) ; キャラクターを動けなくする
        (`self.SetLifeSpan` self 5.0)
        (`self.SetLifeSpan` (`self.EnemyWeaponref`) 5.0) ; 5秒の寿命をつける
        (`PrimitiveComponent.SetCollisionProfileName` (`self.CapsuleComponent`) "NoCollision" true) ; 死亡後に残ったカプセルコンポーネントが余計な\nHit判定を起こさないようにコリジョンプロファイルを変更
      ))
    (else
      (`SceneComponent.SetVisibility` _hp_bar true false) ; HPバー表示
      (`/Game/InGame/Blueprints/Widget/In_Battle/WBP_EnemyHP_Bar.Update HP Bar` (`self.As WBP Enemy HP Bar`)) ; HPバー更新
      (`self.PlayAnimMontage` "/Game/InGame/Animation/Enemies/Montage/Skele_Hit_Montage.Skele_Hit_Montage"))))

(event `Attack`
  ;[1 1 1] 攻撃
  (bind _output_get (set `self.CurrentAttackAnimation` (`KismetArrayLibrary.Array_Random` (`self.AttackAnimation`))))
  (bind _returnvalue (`self.PlayAnimMontage` _output_get))
  (set `self.AttackLength` _returnvalue) ; 攻撃間隔として、攻撃アニメモンタージュの\n長さをAttackLength変数にセット
  (bind _returnvalue_2 (`|GetDataTableRow` "/Game/InGame/Blueprints/Data/DT_EnemySkillData.DT_EnemySkillData" (`KismetStringLibrary.Conv_StringToName` (`KismetSystemLibrary.GetObjectName` _output_get))) ; 配列からランダムで取得したんモンタージュ名から\nスキルデータを取得
    (:`then`
      (bind _output_get_2 (set `self.AttackingSkillData` _returnvalue_2))
      (set `self.Skill Name` (break `/Game/InGame/Blueprints/Data/ST_EnemySkillData` _output_get_2)) ; スキル名をセット
      (if (`KismetStringLibrary.NotEqual_StrStr` (`|GetEnumeratorNameAsString` (`.Type_38_E15B29C740C7F9EEBC8128A58C0B9F4B` (break `/Game/InGame/Blueprints/Data/ST_EnemySkillData` _output_get_2))) "NormalATK")
        (`self.Set WBP_EnemySkillName`) ; 画面に使用中のスキル名を表示
      ))))

(event `Set WBP_EnemySkillName`
  (bind _wbp_skillname (`self.WBP_SkillName`))
  ;[1 1 1] 敵のスキル名表示
  (`UserWidget.AddToViewport` _wbp_skillname 0)
  (`/Game/InGame/Blueprints/Widget/In_Battle/WBP_EnemySkillName.View Enemy Skill Name` _wbp_skillname (`self.Skill Name`))
  (`|PlayAnimation` _wbp_skillname (`/Game/InGame/Blueprints/Widget/In_Battle/WBP_EnemySkillName.Fade` _wbp_skillname) 0.0 1 "Forward" 1.5
    (:`Finished`
      (`Widget.RemoveFromParent` _wbp_skillname))))

(event `Clear Enemies`
  ;[1 1 1] トレースの当たり判定配列をクリア
  ; (二撃目以降の攻撃を有効化)
  (`KismetArrayLibrary.Array_Clear` (`/Game/InGame/Blueprints/Equipment/TraceComponent_Enemeies.ActorToIgnore` (`self.TraceComponent_Enemeies`))))

(event `Event Apply Damage`
  (bind _returnvalue (`KismetMathLibrary.RandomFloatInRange` -5.0 5.0))
  (bind _tracecomponent_enemeies (`self.TraceComponent_Enemeies`))
  (bind (_enemydata_name _enemydata_enemylevel _enemydata_earnexp _enemydata_maxhp _enemydata_hp _enemydata_maxmp _enemydata_mp _enemydata_p_attack) (break `/Game/InGame/Blueprints/Data/ST_EnemyData` (`self.EnemyData`)))
  (bind (_attackingskilldata_skillname _attackingskilldata_atk_multiplier _attackingskilldata_atk_fixvalue) (break `/Game/InGame/Blueprints/Data/ST_EnemySkillData` (`self.AttackingSkillData`)))
  (bind (_player_ref_transform _player_ref_stagelevel _player_ref_name _player_ref_characterlevel _player_ref_totalexp _player_ref_earnexp _player_ref_maxhp _player_ref_hp _player_ref_maxmp _player_ref_mp _player_ref_p_attack _player_ref_m_attack _player_ref_p_defence _player_ref_m_defence _player_ref_def_multiplier) (break `/Game/InGame/Blueprints/Data/ST_PlayerData` (`self.Player Ref`)))
  (bind (_enemyweapondata_name _enemyweapondata_type _enemyweapondata_attackvalue) (break `/Game/InGame/Blueprints/Data/ST_EnemyWeaponData` (`/Game/InGame/Blueprints/Equipment/BP_EnemySword.EnemyWeaponData` (`self.EnemyWeaponref`))))
  (bind _hit_actor (`/Game/InGame/Blueprints/Equipment/TraceComponent_Enemeies.Hit Actor` _tracecomponent_enemeies))
  ;[1 1 1] 武器のトレースにヒットした対象にダメージを与える/ダメージ表示
  (bind _asbp_hero (cast `/Game/InGame/Blueprints/Pawns/Characters/BP_Hero` (`/Game/InGame/Blueprints/Equipment/TraceComponent_Enemeies.Hit Actor` (`self.TraceComponent_Enemeies`))))
  (set `self.Player Ref` (`/Game/InGame/Blueprints/Pawns/Characters/BP_Hero.Player Data` _asbp_hero))
  (bind _returnvalue_2 (`GameplayStatics.ApplyDamage` _hit_actor (- (+ (* (* (+ _enemyweapondata_attackvalue _enemydata_p_attack) (`self.ATKCoefficient`)) _attackingskilldata_atk_multiplier) _attackingskilldata_atk_fixvalue) (* (* (+ _player_ref_p_defence 0.0) (`self.DEFCoefficient`)) _player_ref_def_multiplier)))) ; SwordDamageに設定されたダメージを与える
  (bind _returnvalue_3 (`|SpawnActorFromClass` "/Game/InGame/Blueprints/Widget/In_Battle/BP_DamageValue_ForPlayer.BP_DamageValue_ForPlayer_C" (`KismetMathLibrary.MakeTransform` (+ (`/Game/InGame/Blueprints/Equipment/TraceComponent_Enemeies.Location` _tracecomponent_enemeies) (`KismetMathLibrary.MakeVector` _returnvalue _returnvalue _returnvalue))) "AlwaysSpawn" "MultiplyWithRoot" null null)) ; ダメージ表示ウィジェットをスポーン
  (`/Game/InGame/Blueprints/Widget/In_Battle/BP_DamageValue_ForPlayer.Play Damage Value` _returnvalue_3 (`KismetStringLibrary.Conv_DoubleToString` _returnvalue_2)) ; ダメージ表示
  (`KismetArrayLibrary.Array_Add` (`/Game/InGame/Blueprints/Equipment/TraceComponent_Enemeies.ActorToIgnore` _tracecomponent_enemeies) _hit_actor) ; ActorToIgnore変数の配列にダメージを格納、\nポーン側でクリア
)

(fn `BeginSprint`
  (returns (Succeed :type Boolean))
  (bind _charactermovement (`self.CharacterMovement`))
  (if (`self.IsSprinting`)
    (return false) ; 失敗を返す
    (else
      (set `CharacterMovementComponent.MaxWalkSpeed` (`CharacterMovementComponent.MaxWalkSpeed` _charactermovement) _charactermovement) ; スプリント速度を設定
      (set `self.IsSprinting` true) ; スプリント状態になったら
      (return true) ; 成功を返す
    )))

(fn `BeginWalk`
  (returns (Succeed :type Boolean))
  (bind _charactermovement (`self.CharacterMovement`))
  (if (`self.Is Walking`)
    (return false) ; 失敗を返す
    (else
      (set `CharacterMovementComponent.MaxWalkSpeed` (`CharacterMovementComponent.MaxWalkSpeedCrouched` _charactermovement) _charactermovement) ; 歩行速度を設定
      (set `self.Is Walking` true) ; 歩行状態になった
      (return true) ; 成功を返す
    )))

(fn `EndSprint`
  (returns (Succeed :type Boolean))
  (bind _charactermovement (`self.CharacterMovement`))
  (if (`self.IsSprinting`)
    (set `CharacterMovementComponent.MaxWalkSpeed` (/ (`CharacterMovementComponent.MaxWalkSpeed` _charactermovement) 2.0) _charactermovement) ; 通常歩行時の速度を設定
    (set `self.IsSprinting` false) ; スプリント状態でない
    (return true)
    (else
      (return false) ; 失敗を返す
    )))

(fn `EndWalk`
  (returns (Succeed :type Boolean))
  (if (`self.Is Walking`)
    (set `CharacterMovementComponent.MaxWalkSpeed` 1000.0 (`self.CharacterMovement`)) ; 通常移動時の速度を設定
    (set `self.Is Walking` false) ; 歩行状態でない
    (return true)
    (else
      (return false) ; 失敗を返す
    )))

(fn `Get Is Sprinting`
  (returns (ReturnValue :type Boolean))
  (return (`self.Is Walking`)))

(fn `IsTargetable`
  (returns (ReturnValue :type Boolean))
  (if (< (`self.HP`) 1.0)
    (return false)
    (else
      (return true))))

(fn `UserConstructionScript`)